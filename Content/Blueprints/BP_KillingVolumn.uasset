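; BP_KillingVolumn is a kill volume that removes pickup items entering its Box component.
; On overlap it casts the actor to BP_PickupItem and, if it is a BP_Bowl, first destroys every actor the bowl holds.
; It then reports the item's display name to the task pawn of player 0's BP_Cook for removal from the level's kitchen items, and destroys the item.
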(event OnComponentBeginOverlap(Box)
  (params (OverlappedComponent :type Primitive%20Component%20Object%20Reference) (OtherActor :type Actor%20Object%20Reference) (OtherComp :type Primitive%20Component%20Object%20Reference) (OtherBodyIndex :type Integer) (bFromSweep :type Boolean) (SweepResult :type Hit%20Result%20Structure%20%28by%20ref%29))
  (bind _asbp_pickup_item (Utilities|Casting|CastToBP_PickupItem OtherActor))
  (bind _asbp_cook (Utilities|Casting|CastToBP_Cook (Game|GetPlayerCharacter 0)))
  (bind _asbp_bowl (Utilities|Casting|CastToBP_Bowl _asbp_pickup_item)
    (:then
      (for _array_element (Variables|/Game/Blueprints/BP_Bowl.BP_Bowl_C|GetBowlHoldActors _asbp_bowl)
        (Actor|DestroyActor _array_element)))
    (:CastFailed
      _))
  (Class|TaskPawn|DeleteKitchenIteminLevelItems (Variables|/Game/Blueprints/BP_Cook.BP_Cook_C|GetMyTaskPawn _asbp_cook) (Utilities|GetDisplayName _asbp_pickup_item))
  (Actor|DestroyActor _asbp_pickup_item))

(event EventBeginPlay)

(event Collision|EventActorBeginOverlap
  (params (OtherActor :type Actor%20Object%20Reference)))

(event EventTick
  (params (DeltaSeconds :type Float%20%28single-precision%29)))

(fn ConstructionScript)