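; Game mode for a simple Overcooked-style cooking game, apparently a study build that reports session start, player ID and control value to a remote HTTP server on BeginPlay.
; A delayed Tick counts roughly seconds and shows a paused GameOver screen once two orders succeed or the testing time limit is reached.
; End-of-game timing and statistics uploads are present but disconnected.
; SetLightMode toggles skylight color between black and white; SetBoardMode is empty.
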(event EventBeginPlay
  (Variables|Default|SetGameTimePassed 0)
  (Variables|Default|SetGameSuccessfulOrder 0)
  (bind _asmy_game_instance (Utilities|Casting|CastTomyGameInstance (Game|GetGameInstance)))
  (bind _output_get (Variables|Default|SetRandomID (Variables|/Game/Blueprints/myGameInstance.myGameInstance_C|GetRandomID _asmy_game_instance)))
  (bind _output_get_2 (Variables|Default|Setrequest (Class|VaRestRequestJSON|ConstructRequestExt "GET" "x_www_form_urlencoded_url")))
  (bind _output_get_3 (Variables|Default|SetvaJson (Class|VaRestJsonObject|ConstructJsonObject)))
  (Class|VaRestJsonObject|SetField _output_get_3 "Game Start" (Class|VaRestJsonValue|ConstructJsonValueString "GameStart"))
  (Class|VaRestJsonObject|SetField _output_get_3 "Id" (Class|VaRestJsonValue|ConstructJsonValueString _output_get))
  (Class|VaRestJsonObject|SetField _output_get_3 "Control" (Class|VaRestJsonValue|ConstructJsonValueNumber (Math|Conversions|ToFloat(Integer) (Variables|Default|Getcontrol))))
  (Class|VaRestRequestJSON|SetRequestObject _output_get_2 _output_get_3)
  (Class|VaRestRequestJSON|ProcessURL _output_get_2 "http://stevengong.net:8000"))

(event EventTick
  (params (DeltaSeconds :type Float%20%28single-precision%29))
  (bind _gametimepassed (Variables|Default|GetGameTimePassed))
  (Utilities|FlowControl|Delay 1.0)
  (bind _asbp_cook (Utilities|Casting|CastToBP_Cook (Game|GetPlayerCharacter 0)))
  (Utilities|FlowControl|Sequence
    (:then_0
      (if (>= (Variables|Default|GetGameSuccessfulOrder) 2)
        (bind _returnvalue (UserInterface|CreateWidget "/Game/Blueprints/UI/GameOver.GameOver_C" :!label _label))
        (UserInterface|Viewport|AddtoViewport _returnvalue 0)
        (Variables|/Script/Engine.PlayerController|SetbShowMouseCursor (Game|GetPlayerController 0) true)
        (Game|SetGamePaused true)
        (bind _asbp_cook_2 (Utilities|Casting|CastToBP_Cook (Game|GetPlayerCharacter 0)))
        (Utilities|FlowControl|Sequence)))
    (:then_1
      (Math|Integer|IncrementInt _gametimepassed))
    (:then_2
      (if (>= _gametimepassed (Variables|Default|GettestingMaxTime))
        (goto _label)))))

(fn ConstructionScript)

(fn SetLightMode
  (params (dar :type Boolean) (skyl :type Sky%20Light%20Object%20Reference))
  (bind _lightcomponent (Variables|/Script/Engine.SkyLight|GetLightComponent skyl))
  (if dar
    (Rendering|Components|Light|SetLightColor :self _lightcomponent)
    (else
      (Rendering|Components|Light|SetLightColor _lightcomponent "(R=1.000000,G=1.000000,B=1.000000,A=1.000000)"))))

(fn SetBoardMode)