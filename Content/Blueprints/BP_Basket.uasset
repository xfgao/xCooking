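; BP_Basket is an ingredient dispenser that hands a cook a new food item of its configured ItemName.
; The construction script labels some produce types, while overlap logic here is inactive, with end overlap noted as handled in BP_Cook.
; SpawnGood spawns BP_Food attached to the BasketCollisionActor cook's HoldComponent, sets per-item mesh and properties, and updates holding state.
; It then registers the item through the player cook's MyTaskPawn, noted as a C++ TaskManager interface.
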(event OnComponentBeginOverlap(Box)
  (params (OverlappedComponent :type Primitive%20Component%20Object%20Reference) (OtherActor :type Actor%20Object%20Reference) (OtherComp :type Primitive%20Component%20Object%20Reference) (OtherBodyIndex :type Integer) (bFromSweep :type Boolean) (SweepResult :type Hit%20Result%20Structure%20%28by%20ref%29)))

(event EventBeginPlay)

(event Collision|EventActorBeginOverlap
  (params (OtherActor :type Actor%20Object%20Reference)))

(event EventTick
  (params (DeltaSeconds :type Float%20%28single-precision%29)))

(event Collision|EventActorEndOverlap
  (params (OtherActor :type Actor%20Object%20Reference))
  ;[0.4774 1 0.3175] ~Delete Collision End Overlap Handled in BP_Cook
)

(fn ConstructionScript
  (bind _textrender (Variables|Default|GetTextRender))
  (switch Utilities|FlowControl|Switch|SwitchonFoodList (Variables|Default|GetItemName)
    (:NewEnumerator0
      (Rendering|Components|TextRender|SetText _textrender (LocalVariables|GetCoconut)))
    (:NewEnumerator1
      (Rendering|Components|TextRender|SetText _textrender (LocalVariables|GetGreen%20Apple)))
    (:NewEnumerator2
      (Rendering|Components|TextRender|SetText _textrender (LocalVariables|GetRed%20Apple)))
    (:NewEnumerator3
      (Rendering|Components|TextRender|SetText _textrender (LocalVariables|GetTomato)))
    (:NewEnumerator4
      (Rendering|Components|TextRender|SetText _textrender (LocalVariables|GetTomato)))))

(fn SpawnGood
  (params (who :type BP%20Cook%20Object%20Reference))
  (bind _itemname (Variables|Default|GetItemName))
  ;[1 1 1] Create New Food Item
  (bind _asbp_cook (Utilities|Casting|CastToBP_Cook (Variables|Default|GetBasketCollisionActor)))
  (bind _returnvalue (Game|SpawnActorfromClass "/Game/Blueprints/BP_Food.BP_Food_C" (Transformation|GetWorldTransform (Variables|/Game/Blueprints/BP_Cook.BP_Cook_C|GetHoldComponent _asbp_cook)) "Undefined" 0 0))
  (Transformation|SetActorRelativeScale3D _returnvalue "0.800000,0.800000,0.800000")
  (bind _output_get (Variables|Default|SetNewFood _returnvalue))
  (Physics|SetSimulatePhysics (Variables|/Game/Blueprints/BP_PickupItem.BP_PickupItem_C|GetStaticMesh _returnvalue) false)
  (Collision|SetCollisionEnabled (Variables|/Game/Blueprints/BP_PickupItem.BP_PickupItem_C|GetStaticMesh _returnvalue) "NoCollision")
  (Transformation|AttachComponentToComponent _returnvalue (Variables|/Game/Blueprints/BP_Cook.BP_Cook_C|GetHoldComponent _asbp_cook) "None" "SnapToTarget" "SnapToTarget" "KeepRelative" true)
  (switch Utilities|FlowControl|Switch|SwitchonFoodList _itemname
    (:NewEnumerator0
      (Components|StaticMesh|SetStaticMesh (Variables|/Game/Blueprints/BP_PickupItem.BP_PickupItem_C|GetStaticMesh _returnvalue) "/Game/Assets/food/coconut/coconut_n1.coconut_n1"))
    (:NewEnumerator1
      (Components|StaticMesh|SetStaticMesh (Variables|/Game/Blueprints/BP_PickupItem.BP_PickupItem_C|GetStaticMesh _returnvalue) "/Game/Assets/food/apple_green/Apple_G_n1.Apple_G_n1"))
    (:NewEnumerator2
      (Components|StaticMesh|SetStaticMesh (Variables|/Game/Blueprints/BP_PickupItem.BP_PickupItem_C|GetStaticMesh _returnvalue) "/Game/Assets/food/apple_red/Apple_R_n1.Apple_R_n1"))
    (:NewEnumerator3
      (Components|StaticMesh|SetStaticMesh (Variables|/Game/Blueprints/BP_PickupItem.BP_PickupItem_C|GetStaticMesh _returnvalue) "/Game/Assets/food/lemon/Lemon.Lemon"))
    (:NewEnumerator4
      (Components|StaticMesh|SetStaticMesh (Variables|/Game/Blueprints/BP_PickupItem.BP_PickupItem_C|GetStaticMesh _returnvalue) "/Game/Assets/food/tomato.Tomato")
      (Transformation|SetRelativeRotation (Variables|/Game/Blueprints/BP_PickupItem.BP_PickupItem_C|GetStaticMesh _returnvalue) "0, 0,90.000000" false false)
      (Transformation|SetActorRelativeScale3D (Variables|Default|GetNewFood) "1.200000,1.200000,1.200000"))
    (:NewEnumerator5
      (Components|StaticMesh|SetStaticMesh (Variables|/Game/Blueprints/BP_PickupItem.BP_PickupItem_C|GetStaticMesh _returnvalue) "/Game/Assets/food/meat/meat2.meat2")
      (Variables|/Game/Blueprints/BP_Food.BP_Food_C|SetbFireCookable _returnvalue true))
    (:NewEnumerator6
      (Components|StaticMesh|SetStaticMesh (Variables|/Game/Blueprints/BP_PickupItem.BP_PickupItem_C|GetStaticMesh _returnvalue) "/Game/Assets/food/lettuce_whole.lettuce_whole")
      (Transformation|SetActorRelativeScale3D (Variables|Default|GetNewFood) "0.500000,0.500000,0.500000")
      (Transformation|SetActorRelativeRotation (Variables|Default|GetNewFood) "0, 0,-180.000000"))
    (:NewEnumerator7
      (Components|StaticMesh|SetStaticMesh (Variables|/Game/Blueprints/BP_PickupItem.BP_PickupItem_C|GetStaticMesh _returnvalue) "/Game/Assets/food/bottomBun.bottomBun")
      (Variables|/Game/Blueprints/BP_PickupItem.BP_PickupItem_C|SetbCutable (Variables|Default|GetNewFood) false)
      (Variables|/Game/Blueprints/BP_Food.BP_Food_C|SetbCanPutInBowl (Variables|Default|GetNewFood) true)
      (Transformation|SetActorRelativeScale3D (Variables|Default|GetNewFood) "5.000000,5.000000,5.000000")))
  ;;[1 1 1] Connected to CPP Interface by TaskManager
  (Variables|/Game/Blueprints/BP_Cook.BP_Cook_C|SetCurrentItem _asbp_cook _returnvalue)
  (Variables|/Game/Blueprints/BP_Cook.BP_Cook_C|SetbHoldingItem _asbp_cook true)
  (Variables|/Game/Blueprints/BP_PickupItem.BP_PickupItem_C|SetbHolding _output_get true)
  (Variables|/Game/Blueprints/BP_Food.BP_Food_C|SetFoodName _returnvalue _itemname)
  (bind _asbp_cook_2 (Utilities|Casting|CastToBP_Cook (Game|GetPlayerCharacter 0)))
  (Utilities|FlowControl|Sequence
    (:then_0
      (switch Utilities|FlowControl|Switch|SwitchonFoodList (Variables|Default|GetItemName)
        (:NewEnumerator0
          (Variables|Default|SetNewItemType "ITEM_Cocunut"))
        (:NewEnumerator1
          (Variables|Default|SetNewItemType "ITEM_APPLE_GREEN"))
        (:NewEnumerator2
          (Variables|Default|SetNewItemType "ITEM_APPLE_RED"))
        (:NewEnumerator4
          (Variables|Default|SetNewItemType "ITEM_TOMATO"))
        (:NewEnumerator5
          (Variables|Default|SetNewItemType "ITEM_MEAT"))
        (:NewEnumerator6
          (Variables|Default|SetNewItemType "ITEM_LETTUCE"))
        (:NewEnumerator7
          (Variables|Default|SetNewItemType "ITEM_BREAD"))))
    (:then_1
      (Class|TaskPawn|AddNewKitchenItemtoLevelItems (Variables|/Game/Blueprints/BP_Cook.BP_Cook_C|GetMyTaskPawn _asbp_cook_2) (Utilities|GetDisplayName (Variables|Default|GetNewFood)) (Variables|Default|GetNewItemType) "BE_HOLD" (Variables|/Game/Blueprints/BP_Cook.BP_Cook_C|GetCookType _asbp_cook)))))