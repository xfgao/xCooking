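; Game instance Blueprint that generates a time-based RandomID for the Simple Overcooked game when it initializes.
; On Init, it concatenates the current date and time, from year down to millisecond, into an unpadded string and prints it.
; It then casts the current game mode to SimpleOvercookedGameMode and copies the ID there, doing nothing further if the cast fails.
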(event EventInit
  (bind _returnvalue (Math|DateTime|Now))
  (bind (_year _month _day _hour _minute _second _millisecond) (Math|DateTime|BreakDateTime _returnvalue))
  (bind _output_get (Variables|Default|SetRandomID (Utilities|String|Append (Utilities|String|ToString(Integer) _year) (Utilities|String|ToString(Integer) _month) (Utilities|String|ToString(Integer) _day) (Utilities|String|ToString(Integer) _hour) (Utilities|String|ToString(Integer) _minute) (Utilities|String|ToString(Integer) _second) (Utilities|String|ToString(Integer) _millisecond))))
  (Development|PrintString _output_get)
  (bind _assimple_overcooked_game_mode (Utilities|Casting|CastToSimpleOvercookedGameMode (Game|GetGameMode)))
  (Variables|/Game/Blueprints/SimpleOvercookedGameMode.SimpleOvercookedGameMode_C|SetRandomID _assimple_overcooked_game_mode _output_get))