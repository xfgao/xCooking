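; Cabinet actor that supplies cups: SpawnCup spawns a BP_Cup at the hold component of the cook stored in CabinetCollisionActor.
; The cup is scaled down, made non-cutable with physics and collision off, attached to that component and set as the cook's held item.
; It is also logged in the task pawn's LevelItems as a held BOWL, as a link to C++.
; The event graph is inactive, with end-overlap handling left to BP_Cook.
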(event EventBeginPlay)

(event Collision|EventActorBeginOverlap
  (params (OtherActor :type Actor%20Object%20Reference)))

(event EventTick
  (params (DeltaSeconds :type Float%20%28single-precision%29)))

(event Collision|EventActorEndOverlap
  (params (OtherActor :type Actor%20Object%20Reference))
  ;[0.4774 1 0.3175] ~Delete Collision End Overlap Handled in BP_Cook
)

(fn ConstructionScript)

(fn SpawnCup
  (params (who :type ECOOKTYPE%20Enum :default "PLAYER"))
  ;[1 1 1] Spawn Bowl/Plate/Bottle
  (bind _asbp_cook (Utilities|Casting|CastToBP_Cook (Variables|Default|GetCabinetCollisionActor)))
  (bind _returnvalue (Game|SpawnActorfromClass "/Game/Blueprints/BP_Cup.BP_Cup_C" (Transformation|GetWorldTransform (Variables|/Game/Blueprints/BP_Cook.BP_Cook_C|GetHoldComponent _asbp_cook)) "Undefined" 0 0))
  (Transformation|SetActorRelativeScale3D _returnvalue "0.200000,0.200000,0.200000")
  (Physics|SetSimulatePhysics (Variables|/Game/Blueprints/BP_PickupItem.BP_PickupItem_C|GetStaticMesh _returnvalue) false)
  (Collision|SetCollisionEnabled (Variables|/Game/Blueprints/BP_PickupItem.BP_PickupItem_C|GetStaticMesh _returnvalue) "NoCollision")
  (Variables|/Game/Blueprints/BP_PickupItem.BP_PickupItem_C|SetbCutable _returnvalue false)
  (Transformation|AttachComponentToComponent (Variables|/Game/Blueprints/BP_PickupItem.BP_PickupItem_C|GetStaticMesh _returnvalue) (Variables|/Game/Blueprints/BP_Cook.BP_Cook_C|GetHoldComponent _asbp_cook) "None" "SnapToTarget" "SnapToTarget" "KeepWorld" true)
  (Variables|/Game/Blueprints/BP_Cook.BP_Cook_C|SetbHoldingItem _asbp_cook true)
  (Variables|/Game/Blueprints/BP_Cook.BP_Cook_C|SetCurrentItem _asbp_cook _returnvalue)
  ;[1 1 1] Link to CPP file
  (Utilities|Array|Add (Variables|/Script/SimpleOvercooked.TaskPawn|GetLevelItems (Variables|/Game/Blueprints/BP_Cook.BP_Cook_C|GetMyTaskPawn _asbp_cook)) (Utilities|Struct|MakeKitchenItem (Utilities|GetDisplayName _returnvalue) "ITEM_BOWL" (LocalVariables|GetTestNoneArray) (Math|Transform|MakeTransform "0, 0, 0") "BE_HOLD"))
  (bind _asbp_cook_2 (Utilities|Casting|CastToBP_Cook (Game|GetPlayerCharacter 0))))