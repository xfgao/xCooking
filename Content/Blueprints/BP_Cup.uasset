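; BP_Cup is a kitchen container that receives food items in a cooking game, reusing bowl-named logic.
; GetFoodInBowl records the food as held, turns off its physics and collision, snaps it to ContainComp and increments the item count.
; It then has the player cook's task pawn add the food as a cup attribute with its cook type and remove it from level items.
; DropBowl is an empty stub with disconnected throw logic.
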(event EventBeginPlay)

(event Collision|EventActorBeginOverlap
  (params (OtherActor :type Actor%20Object%20Reference)))

(event EventTick
  (params (DeltaSeconds :type Float%20%28single-precision%29)))

(fn ConstructionScript)

(fn DropBowl
  ;[0.2719 1 0.1332] ~Delete
)

(fn GetFoodinBowl
  (params (food :type BP%20Food%20Object%20Reference) (who :type BP%20Cook%20Object%20Reference))
  (bind _returnvalue (Utilities|GetDisplayName food))
  (bind _staticmesh (Variables|/Game/Blueprints/BP_PickupItem.BP_PickupItem_C|GetStaticMesh food))
  (bind _containcomp (Variables|Default|GetContainComp))
  (Utilities|FlowControl|Sequence
    (:then_0
      ;[1 1 1] AttachFood to Bowl
      (Utilities|Array|Add (Variables|Default|GetBowlHoldActors) food)
      (Variables|/Game/Blueprints/BP_PickupItem.BP_PickupItem_C|SetbHolding food true)
      (Transformation|DetachFromComponent _staticmesh "KeepWorld" "KeepWorld" "KeepRelative" true)
      (Rendering|SetVisibility _staticmesh true false)
      (Physics|SetSimulatePhysics _staticmesh false)
      (Collision|SetCollisionEnabled _staticmesh "NoCollision")
      (Transformation|AttachComponentToComponent _staticmesh _containcomp "None" "SnapToTarget" "KeepRelative" "KeepRelative" true)
      (Transformation|AddRelativeRotation _containcomp (Math|Rotator|MakeRotator 0.0 0.0 (* 0 4e+01)) false false)
      (Variables|Default|SetitemNum (+ (Variables|Default|GetitemNum) 1)))
    (:then_1
      (bind _asbp_cook (Utilities|Casting|CastToBP_Cook (Game|GetPlayerCharacter 0)))
      ;[1 1 1] Cpp
      (Class|TaskPawn|AddKitchenItemAttribute (Variables|/Game/Blueprints/BP_Cook.BP_Cook_C|GetMyTaskPawn _asbp_cook) (Utilities|GetDisplayName self) _returnvalue (Variables|/Game/Blueprints/BP_Cook.BP_Cook_C|GetCookType who))
      (Class|TaskPawn|DeleteKitchenIteminLevelItems (Variables|/Game/Blueprints/BP_Cook.BP_Cook_C|GetMyTaskPawn _asbp_cook) _returnvalue))))