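; Cutting board station that holds one pickup item and lets a cook slice coconuts and red or green apples.
; Box overlap snaps a free item onto the board, and Tick clears the slot once it leaves.
; Cut puts the knife in the cook's hand, locks player input and runs a timeline-driven progress bar, then swaps to the sliced mesh.
; Occupancy, item location and cut type are reported to the C++ MyTaskPawn for task tracking.
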(event OnComponentBeginOverlap(Box)
  (params (OverlappedComponent :type Primitive%20Component%20Object%20Reference) (OtherActor :type Actor%20Object%20Reference) (OtherComp :type Primitive%20Component%20Object%20Reference) (OtherBodyIndex :type Integer) (bFromSweep :type Boolean) (SweepResult :type Hit%20Result%20Structure%20%28by%20ref%29))
  (bind _returnvalue (Utilities|GetDisplayName OtherActor))
  ;[1 1 1] Collision
  (if (not (Variables|Default|GetCutboardOccupied))
    (bind _asbp_pickup_item (Utilities|Casting|CastToBP_PickupItem OtherActor))
    (if (not (Variables|/Game/Blueprints/BP_PickupItem.BP_PickupItem_C|GetbHolding _asbp_pickup_item))
      (if (not (Variables|/Game/Blueprints/BP_PickupItem.BP_PickupItem_C|GetbOnGrid _asbp_pickup_item))
        (Physics|SetSimulatePhysics (Variables|/Game/Blueprints/BP_PickupItem.BP_PickupItem_C|GetStaticMesh _asbp_pickup_item) false)
        (Collision|SetCollisionEnabled (Variables|/Game/Blueprints/BP_PickupItem.BP_PickupItem_C|GetStaticMesh _asbp_pickup_item) "NoCollision")
        (Transformation|SetActorLocation _asbp_pickup_item (Transformation|GetWorldLocation (Variables|Default|GetBox)) false true)
        (Transformation|SetActorRotation _asbp_pickup_item (Transformation|GetActorRotation) true)
        (Variables|Default|SetCutboardOccupied true)
        (Variables|/Game/Blueprints/BP_PickupItem.BP_PickupItem_C|SetbOnGrid _asbp_pickup_item true)
        (Variables|Default|SetCutBoardItem _asbp_pickup_item)
        (Collision|SetCollisionEnabled (Variables|/Game/Blueprints/BP_PickupItem.BP_PickupItem_C|GetStaticMesh _asbp_pickup_item) "QueryAndPhysics")
        ;[1 1 1] Cpp: change occupation for table
        (bind _asbp_cook (Utilities|Casting|CastToBP_Cook (Game|GetPlayerCharacter 0)))
        (Class|TaskPawn|ChangeToolOccupation (Variables|/Game/Blueprints/BP_Cook.BP_Cook_C|GetMyTaskPawn _asbp_cook) (Utilities|GetDisplayName self) true)
        ;[1 1 1] Set Instruction Widget Visibility
        (Rendering|SetVisibility (Variables|Default|GetWidget) false false)
        (bind _asbp_cook_2 (Utilities|Casting|CastToBP_Cook (Game|GetPlayerCharacter 0)))
        (Class|TaskPawn|ChangeItemAbstractLocation (Variables|/Game/Blueprints/BP_Cook.BP_Cook_C|GetMyTaskPawn _asbp_cook_2) _returnvalue "ON_CUTBOARD")
        (Class|TaskPawn|ChangeFluent (Variables|/Game/Blueprints/BP_Cook.BP_Cook_C|GetMyTaskPawn _asbp_cook_2) (Variables|Default|GetCutType) "ON_CUTBOARD" "PLAYER" _returnvalue)))))

(event Custom|Cut
  (params (who :type BP%20Cook%20Object%20Reference))
  (bind _progresswidgetcomp (Variables|Default|GetProgressWidgetComp))
  (bind _knife (Variables|Default|GetKnife))
  (bind _cutboarditem (Variables|Default|GetCutBoardItem))
  (bind _returnvalue (Utilities|GetDisplayName _cutboarditem))
  ;[1 1 1] Cut Food
  (if (!= _cutboarditem 0)
    (bind _asbp_food (Utilities|Casting|CastToBP_Food _cutboarditem))
    (if (Variables|/Game/Blueprints/BP_PickupItem.BP_PickupItem_C|GetbCutable _asbp_food)
      (Variables|/Game/Blueprints/BP_PickupItem.BP_PickupItem_C|SetbCutable _asbp_food false)
      (bind _asbp_cook (Utilities|Casting|CastToBP_Cook (Variables|Default|GetCookToolCollisionActor)))
      (bind _asprogress_bar_widget (Utilities|Casting|CastToProgressBarWidget (UserInterface|GetUserWidgetObject _progresswidgetcomp)))
      (Variables|/Game/Blueprints/BP_Cook.BP_Cook_C|SetbCanMove _asbp_cook false)
      (Rendering|ToggleVisibility _progresswidgetcomp false)
      (bind _output_get (Variables|Default|SetKnifeTransform (Transformation|GetWorldTransform _knife)))
      (Transformation|AttachComponentToComponent _knife (Variables|/Script/Engine.Character|GetMesh _asbp_cook) "hand_socket_r" "SnapToTarget" "SnapToTarget" "KeepWorld" false)
      (Input|DisableInput (Game|GetPlayerCharacter 0) (Game|GetPlayerController 0))
      (bind _progress (Timeline|CutTIme PlayFromStart)
        (:Update
          (Variables|/Game/Blueprints/BP_Cook.BP_Cook_C|SetbCutting _asbp_cook true)
          (Progress|SetPercent (Variables|/Game/Blueprints/UI/ProgressBarWidget.ProgressBarWidget_C|GetProgressBar_53 _asprogress_bar_widget) _progress))
        (:Finished
          ;[1 1 1] Set New mesh
          (Variables|/Game/Blueprints/BP_Cook.BP_Cook_C|SetbCanMove _asbp_cook true)
          (Variables|/Game/Blueprints/BP_Cook.BP_Cook_C|SetbCutting _asbp_cook false)
          (Rendering|ToggleVisibility _progresswidgetcomp false)
          (Transformation|DetachFromComponent _knife "KeepRelative" "KeepRelative" "KeepRelative" true)
          (Transformation|SetWorldTransform _knife _output_get false false)
          (Utilities|FlowControl|Sequence
            (:then_0
              (switch Utilities|FlowControl|Switch|SwitchonFoodList (Variables|/Game/Blueprints/BP_Food.BP_Food_C|GetFoodName _asbp_food)
                (:NewEnumerator0
                  (Components|StaticMesh|SetStaticMesh (Variables|/Game/Blueprints/BP_PickupItem.BP_PickupItem_C|GetStaticMesh _asbp_food) "/Game/Assets/food/coconut/Coconut_Cut.Coconut_Cut")
                  (Variables|Default|SetCutType "ITEM_SLICED_Cocunut"))
                (:NewEnumerator1
                  (Components|StaticMesh|SetStaticMesh (Variables|/Game/Blueprints/BP_PickupItem.BP_PickupItem_C|GetStaticMesh _asbp_food) "/Game/Assets/food/apple_green/Apple_G_Cut_n1.Apple_G_Cut_n1")
                  (Variables|Default|SetCutType "ITEM_SLICED_APPLE_GREEN"))
                (:NewEnumerator2
                  (Components|StaticMesh|SetStaticMesh (Variables|/Game/Blueprints/BP_PickupItem.BP_PickupItem_C|GetStaticMesh _asbp_food) "/Game/Assets/food/apple_red/Apple_R_Cut_n1.Apple_R_Cut_n1")
                  (Variables|Default|SetCutType "ITEM_SLICED_APPLE_RED")))
              (Variables|/Game/Blueprints/BP_PickupItem.BP_PickupItem_C|SetbCutable _asbp_food false)
              (Variables|/Game/Blueprints/BP_Food.BP_Food_C|SetbCanPutInBowl _asbp_food false)
              (Variables|/Game/Blueprints/BP_Food.BP_Food_C|SetbCanPutInJuicer _asbp_food true)
              (Variables|/Game/Blueprints/BP_Cook.BP_Cook_C|SetCollisionActor who _asbp_food)
              (Variables|/Game/Blueprints/BP_PickupItem.BP_PickupItem_C|SetPickUpCollisionActor _asbp_food who)
              (bind _asbp_cook_2 (Utilities|Casting|CastToBP_Cook (Game|GetPlayerCharacter 0)))
              (Class|TaskPawn|ChangeItemAbstractLocation (Variables|/Game/Blueprints/BP_Cook.BP_Cook_C|GetMyTaskPawn _asbp_cook_2) _returnvalue "ON_CUTBOARD")
              (Class|TaskPawn|ChangeFluent (Variables|/Game/Blueprints/BP_Cook.BP_Cook_C|GetMyTaskPawn _asbp_cook_2) (Variables|Default|GetCutType) "ON_CUTBOARD" (Variables|/Game/Blueprints/BP_Cook.BP_Cook_C|GetCookType who) _returnvalue)
              (bind _asbp_cook_3 (Utilities|Casting|CastToBP_Cook (Game|GetPlayerCharacter 0)))
              (bind _returnvalue_2 (Class|TaskPawn|CheckItemPlayer (Variables|/Game/Blueprints/BP_Cook.BP_Cook_C|GetMyTaskPawn _asbp_cook_3)))
              (if _returnvalue_2
                (Class|TaskPawn|UpdateAOGHuman (Variables|/Game/Blueprints/BP_Cook.BP_Cook_C|GetMyTaskPawn _asbp_cook_3))
                (Class|TaskPawn|ExplainAOGHuman (Variables|/Game/Blueprints/BP_Cook.BP_Cook_C|GetMyTaskPawn _asbp_cook_3)))
              (Input|EnableInput (Game|GetPlayerCharacter 0) (Game|GetPlayerController 0)))
            (:then_1
              ;[1 1 1] Cpp
              (Class|TaskPawn|ChangeKitchenItemType (Variables|/Game/Blueprints/BP_Cook.BP_Cook_C|GetMyTaskPawn _asbp_cook) (Utilities|GetDisplayName _asbp_food) (Variables|Default|GetCutType) (Variables|/Game/Blueprints/BP_Cook.BP_Cook_C|GetCookType who)))))))))

(event EventBeginPlay)

(event Collision|EventActorBeginOverlap
  (params (OtherActor :type Actor%20Object%20Reference)))

(event EventTick
  (params (DeltaSeconds :type Float%20%28single-precision%29))
  ;[1 1 1] Collision
  (if (!= (Variables|Default|GetCutBoardItem) 0)
    (if (or (Variables|/Game/Blueprints/BP_PickupItem.BP_PickupItem_C|GetbHolding (Variables|Default|GetCutBoardItem)) (not (Variables|/Game/Blueprints/BP_PickupItem.BP_PickupItem_C|GetbOnGrid (Variables|Default|GetCutBoardItem))))
      (Variables|Default|SetCutBoardItem 0)
      (Variables|Default|SetCutboardOccupied false)
      ;;[1 1 1] Cpp: change occupation for table
      (bind _asbp_cook (Utilities|Casting|CastToBP_Cook (Game|GetPlayerCharacter 0)))
      (Class|TaskPawn|ChangeToolOccupation (Variables|/Game/Blueprints/BP_Cook.BP_Cook_C|GetMyTaskPawn _asbp_cook) (Utilities|GetDisplayName self) false)
      ;;[1 1 1] Set Instruction Widget Visibility
      (Rendering|SetVisibility (Variables|Default|GetWidget) true false))))

(fn ConstructionScript)