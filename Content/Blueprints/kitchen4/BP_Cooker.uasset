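; BP_Cooker is a kitchen pan that holds one pickup item and fire-cooks the food on it.
; A loose item overlapping the box snaps onto the pan, and Tick frees the pan once that item is held or off-grid.
; FireCook locks cookable food and runs a timeline-driven progress bar.
; On finish, meat switches to a burger mesh, becomes bowl-ready, reports its cooked type to the cook's C++ task pawn and unlocks for pickup.
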(event OnComponentBeginOverlap(Box)
  (params (OverlappedComponent :type Primitive%20Component%20Object%20Reference) (OtherActor :type Actor%20Object%20Reference) (OtherComp :type Primitive%20Component%20Object%20Reference) (OtherBodyIndex :type Integer) (bFromSweep :type Boolean) (SweepResult :type Hit%20Result%20Structure%20%28by%20ref%29))
  ;[1 1 1] Collision: Pickup item on Pan
  (if (not (Variables|Default|GetPanOccupied))
    (bind _asbp_pickup_item (Utilities|Casting|CastToBP_PickupItem OtherActor))
    (if (not (Variables|/Game/Blueprints/BP_PickupItem.BP_PickupItem_C|GetbHolding _asbp_pickup_item))
      (if (not (Variables|/Game/Blueprints/BP_PickupItem.BP_PickupItem_C|GetbOnGrid _asbp_pickup_item))
        (Physics|SetSimulatePhysics (Variables|/Game/Blueprints/BP_PickupItem.BP_PickupItem_C|GetStaticMesh _asbp_pickup_item) false)
        (Collision|SetCollisionEnabled (Variables|/Game/Blueprints/BP_PickupItem.BP_PickupItem_C|GetStaticMesh _asbp_pickup_item) "NoCollision")
        (Transformation|SetActorLocation _asbp_pickup_item (Transformation|GetWorldLocation (Variables|Default|GetBox)) false true)
        (Variables|Default|SetPanOccupied true)
        (Variables|/Game/Blueprints/BP_PickupItem.BP_PickupItem_C|SetbOnGrid _asbp_pickup_item true)
        (Variables|Default|SetPanItem _asbp_pickup_item)
        (Collision|SetCollisionEnabled (Variables|/Game/Blueprints/BP_PickupItem.BP_PickupItem_C|GetStaticMesh _asbp_pickup_item) "QueryOnly")))))

(event Custom|FireCook
  (params (who :type BP%20Cook%20Object%20Reference))
  (bind _progresswidgetcomp (Variables|Default|GetProgressWidgetComp))
  (bind _panitem (Variables|Default|GetPanItem))
  (if (!= _panitem 0)
    (bind _asbp_food (Utilities|Casting|CastToBP_Food _panitem))
    (if (Variables|/Game/Blueprints/BP_Food.BP_Food_C|GetbFireCookable _asbp_food)
      (Variables|/Game/Blueprints/BP_PickupItem.BP_PickupItem_C|SetbCanPickedUp _asbp_food false)
      (Variables|/Game/Blueprints/BP_Food.BP_Food_C|SetbFireCookable _asbp_food false)
      (bind _asprogress_bar_widget (Utilities|Casting|CastToProgressBarWidget (UserInterface|GetUserWidgetObject _progresswidgetcomp)))
      (Rendering|ToggleVisibility _progresswidgetcomp false)
      (bind _progress (Timeline|Timeline_0 PlayFromStart)
        (:Update
          (Progress|SetPercent (Variables|/Game/Blueprints/UI/ProgressBarWidget.ProgressBarWidget_C|GetProgressBar_53 _asprogress_bar_widget) _progress))
        (:Finished
          (Rendering|ToggleVisibility _progresswidgetcomp false)
          (switch Utilities|FlowControl|Switch|SwitchonFoodList (Variables|/Game/Blueprints/BP_Food.BP_Food_C|GetFoodName _asbp_food)
            (:NewEnumerator5
              (Components|StaticMesh|SetStaticMesh (Variables|/Game/Blueprints/BP_PickupItem.BP_PickupItem_C|GetStaticMesh _asbp_food) "/Game/Assets/food/burger_meat.burger_meat")
              (Variables|/Game/Blueprints/BP_Food.BP_Food_C|SetbCanPutInBowl _asbp_food true)
              (Variables|Default|SetPanCookedType "ITEM_COOKED_MEAT")
              ;[0.1687 0.05208 1] CPP Information Transfer: Pan
              (bind _asbp_cook (Utilities|Casting|CastToBP_Cook (Variables|Default|GetCookToolCollisionActor)))
              (Class|TaskPawn|ChangeKitchenItemType (Variables|/Game/Blueprints/BP_Cook.BP_Cook_C|GetMyTaskPawn _asbp_cook) (Utilities|GetDisplayName _asbp_food) (Variables|Default|GetPanCookedType) (Variables|/Game/Blueprints/BP_Cook.BP_Cook_C|GetCookType _asbp_cook))
              (Variables|/Game/Blueprints/BP_PickupItem.BP_PickupItem_C|SetbCanPickedUp _asbp_food true))))))))

(event EventBeginPlay
  (|CallParentFunction) ; This node is disabled and will not be called.\nDrag off pins to build functionality.
)

(event Collision|EventActorBeginOverlap
  (params (OtherActor :type Actor%20Object%20Reference))
  (|CallParentFunction OtherActor) ; This node is disabled and will not be called.\nDrag off pins to build functionality.
)

(event EventTick
  (params (DeltaSeconds :type Float%20%28single-precision%29))
  (|CallParentFunction DeltaSeconds)
  (if (!= (Variables|Default|GetPanItem) 0)
    (if (or (Variables|/Game/Blueprints/BP_PickupItem.BP_PickupItem_C|GetbHolding (Variables|Default|GetPanItem)) (not (Variables|/Game/Blueprints/BP_PickupItem.BP_PickupItem_C|GetbOnGrid (Variables|Default|GetPanItem))))
      (Variables|Default|SetPanItem 0)
      (Variables|Default|SetPanOccupied false))))

(fn ConstructionScript
  (|CallParentFunction))