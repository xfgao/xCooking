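; AI robot cook for the kitchen4 level; live logic only sets walk speed and cook type, idles its task pawn, hides a scene component and saves its start transform.
; A disconnected state machine, with Tick left empty, would execute MyTaskPawn's move, pick-up/drop and operate actions on name-matched targets and report results for replanning.
; It also holds idle item scanning within fixed bounds and retreat-on-failure near the start.
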(event EventBeginPlay
  ;[1 1 1] Set Max Movement Speed for AI
  (|CallParentFunction)
  (Variables|/Script/Engine.CharacterMovementComponent|SetMaxWalkSpeed (Variables|Character|GetCharacterMovement self) 2.7e+02)
  (Variables|Default|SetCookType "ROBOT")
  (Utilities|FlowControl|Delay 0.2)
  (Variables|/Script/SimpleOvercooked.TaskPawn|SetAIAction (Variables|Default|GetMyTaskPawn) "IDLE")
  (Rendering|SetVisibility (Variables|Default|GetScene) false true)
  (Variables|Default|SetOriginalTransform (Transformation|GetActorTransform)))

(event Collision|EventActorBeginOverlap
  (params (OtherActor :type Actor%20Object%20Reference))
  (|CallParentFunction OtherActor) ; This node is disabled and will not be called.\nDrag off pins to build functionality.
)

(event EventTick
  (params (DeltaSeconds :type Float%20%28single-precision%29)))

(fn ConstructionScript
  (|CallParentFunction))

(fn FindPickItem2MiddleTable(1-2Only)
  (bind _outactors (Actor|GetAllActorsOfClass "/Script/Engine.Actor"))
  (bind _array_element (Utilities|Array|ForEachLoopwithBreak _outactors)
    (:LoopBody
      (bind _asbp_pickup_item (Utilities|Casting|CastToBP_PickupItem _array_element))
      (if (and (< (.X (Math|Vector|BreakVector (Transformation|GetActorLocation _asbp_pickup_item))) 4e+02) (> (.X (Math|Vector|BreakVector (Transformation|GetActorLocation _asbp_pickup_item))) 1.1e+02))
        (if (and (< (.Y (Math|Vector|BreakVector (Transformation|GetActorLocation _asbp_pickup_item))) 4.7e+02) (> (.Y (Math|Vector|BreakVector (Transformation|GetActorLocation _asbp_pickup_item))) -4.7e+02))
          (if (and (Utilities|Enum|NotEqual(Enum) (Variables|/Game/Blueprints/BP_PickupItem.BP_PickupItem_C|GetAbstractLocation _asbp_pickup_item) "BE_HOLD") (Utilities|Enum|NotEqual(Enum) (Variables|/Game/Blueprints/BP_PickupItem.BP_PickupItem_C|GetAbstractLocation _asbp_pickup_item) "ON_TABLE"))
            (return _asbp_pickup_item)))))
    (:Completed
      (return 0))))