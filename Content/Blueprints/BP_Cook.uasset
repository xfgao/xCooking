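; Cook character for an Overcooked-style game, drivable by player input or AI events.
; A box overlap caches the nearby interactable and cook tool, linking them back to the cook.
; Pickup/drop, shared by input and AI, casts these to handle food, bowls, baskets, cabinets and trash; Operate triggers cutting, cooking or juicing, with a narrower AI variant.
; It also handles axis-snapped movement, tracks idle time and reports held items for AI planning.
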(event Custom|AIOperate
  (bind _currentcooktool (Variables|Default|GetCurrentCookTool))
  (if (not (Variables|Default|GetbHoldingItem))
    (if (!= _currentcooktool 0)
      (bind _asbp_cutboard (Utilities|Casting|CastToBP_Cutboard _currentcooktool)
        (:then
          (Default|Cut _asbp_cutboard self))
        (:CastFailed
          (bind _as1_1_juicer (Utilities|Casting|CastTo1-1_Juicer _currentcooktool))
          (Default|MakeJuice _as1_1_juicer self)))
      (bind _returnvalue (Game|GetCurrentLevelName true))
      (if (Utilities|Enum|NotEqual(Enum) _returnvalue "training")
        _))))

(event Custom|AIPickUpDrop
  (bind _collisionactor (Variables|Default|GetCollisionActor))
  (bind _collisionactor_2 (Variables|Default|GetCollisionActor))
  (Utilities|FlowControl|Sequence
    (:then_0
      (if (Variables|Default|GetbHoldingItem)
        (bind _asbp_trashbin (Utilities|Casting|CastToBP_Trashbin _collisionactor_2)
          (:then
            (Default|Dump _asbp_trashbin)
            (Variables|Default|SetCurrentItem 0 :!label _label)
            (Variables|Default|SetbHoldingItem false))
          (:CastFailed
            (bind _asbp_bowl (Utilities|Casting|CastToBP_Bowl (Variables|Default|GetCurrentItem))
              (:then
                (bind _asbp_food (Utilities|Casting|CastToBP_Food _collisionactor_2)
                  (:then
                    (if (Variables|/Game/Blueprints/BP_Food.BP_Food_C|GetbCanPutInBowl _asbp_food)
                      (if (not (Variables|/Game/Blueprints/BP_PickupItem.BP_PickupItem_C|GetbHolding _asbp_food))
                        (Default|GetFoodinBowl _asbp_bowl _asbp_food self)
                        (Variables|/Game/Blueprints/BP_PickupItem.BP_PickupItem_C|SetbOnGrid _asbp_food false)
                        (Variables|/Game/Blueprints/BP_PickupItem.BP_PickupItem_C|SetbHolding _asbp_food true))
                      (else
                        (Default|Drop (Variables|Default|GetCurrentItem) (Utilities|GetDisplayName (Variables|Default|GetCurrentItem)) (Variables|Default|GetCookType) :!label _label_2)
                        (goto _label))))
                  (:CastFailed
                    (goto _label_2))))
              (:CastFailed
                ;[1 1 1] 如果是食物，判断是扔掉还是放进盘子里，放进盘里的东西不能拿出来
                (bind _asbp_food_2 (Utilities|Casting|CastToBP_Food (Variables|Default|GetCurrentItem)))
                (if (Variables|/Game/Blueprints/BP_Food.BP_Food_C|GetbCanPutInBowl _asbp_food_2)
                  (bind _asbp_bowl_2 (Utilities|Casting|CastToBP_Bowl (Variables|Default|GetCollisionActor))
                    (:then
                      (Development|PrintString "BOWLLLLLLLLLLLLLLLLLLLLLLLLLL")
                      (Default|GetFoodinBowl _asbp_bowl_2 _asbp_food_2 self)
                      (goto _label))
                    (:CastFailed
                      (goto _label_2)))
                  (else
                    (goto _label_2)))))))
        (else
          (bind _asbp_basket (Utilities|Casting|CastToBP_Basket _collisionactor)
            (:then
              (if (not (Variables|/Game/Blueprints/BP_Basket.BP_Basket_C|GetHasItem _asbp_basket))
                (Default|SpawnGood _asbp_basket self)))
            (:CastFailed
              (bind _asbp_food_3 (Utilities|Casting|CastToBP_Food _collisionactor)
                (:then
                  (if (not (Variables|/Game/Blueprints/BP_Food.BP_Food_C|GetbMustPutInBowl _asbp_food_3))
                    (if (not (Variables|/Game/Blueprints/BP_PickupItem.BP_PickupItem_C|GetbHolding _asbp_food_3))
                      (Default|PickUp2 _asbp_food_3 (Variables|Default|GetCookType)))))
                (:CastFailed
                  (bind _asbp_pickup_item (Utilities|Casting|CastToBP_PickupItem _collisionactor)
                    (:then
                      (Default|PickUp2 _asbp_pickup_item (Variables|Default|GetCookType)))
                    (:CastFailed
                      (bind _asbp_cabinet (Utilities|Casting|CastToBP_Cabinet _collisionactor))
                      (Default|SpawnBowl _asbp_cabinet (Variables|Default|GetCookType))
                      (if (Utilities|Enum|Equal(Enum) (Variables|Default|GetCookType) "PLAYER")
                        _))))))))))))

(event EventBeginPlay)

(event Collision|EventActorBeginOverlap
  (params (OtherActor :type Actor%20Object%20Reference)))

(event EventTick
  (params (DeltaSeconds :type Float%20%28single-precision%29))
  (Variables|Default|SetTimeNoInput (+ DeltaSeconds (Variables|Default|GetTimeNoInput))))

(event Input|ActionEvents|InputActionPickUpDrop
  (params (Key :type Key%20Structure :default "None"))
  (bind _collisionactor (Variables|Default|GetCollisionActor))
  (bind _collisionactor_2 (Variables|Default|GetCollisionActor))
  ;[1 1 1] E click: Pickup Drop
  (:Pressed
    (Variables|Default|SetTimeNoInput 0.0)
    (Utilities|FlowControl|Sequence
      (:then_0
        (if (Variables|Default|GetbHoldingItem)
          (bind _asbp_trashbin (Utilities|Casting|CastToBP_Trashbin _collisionactor_2)
            (:then
              (Default|Dump _asbp_trashbin)
              (Variables|Default|SetCurrentItem 0 :!label _label)
              (Variables|Default|SetbHoldingItem false))
            (:CastFailed
              (bind _asbp_bowl (Utilities|Casting|CastToBP_Bowl (Variables|Default|GetCurrentItem))
                (:then
                  (bind _asbp_food (Utilities|Casting|CastToBP_Food _collisionactor_2)
                    (:then
                      (if (Variables|/Game/Blueprints/BP_Food.BP_Food_C|GetbCanPutInBowl _asbp_food)
                        (if (not (Variables|/Game/Blueprints/BP_PickupItem.BP_PickupItem_C|GetbHolding _asbp_food))
                          (Default|GetFoodinBowl _asbp_bowl _asbp_food self)
                          (Variables|/Game/Blueprints/BP_PickupItem.BP_PickupItem_C|SetbOnGrid _asbp_food false)
                          (Variables|/Game/Blueprints/BP_PickupItem.BP_PickupItem_C|SetbHolding _asbp_food true))
                        (else
                          (Default|Drop (Variables|Default|GetCurrentItem) (Utilities|GetDisplayName (Variables|Default|GetCurrentItem)) (Variables|Default|GetCookType) :!label _label_2)
                          (goto _label))))
                    (:CastFailed
                      (goto _label_2))))
                (:CastFailed
                  ;[1 1 1] 如果是食物，判断是扔掉还是放进盘子里，放进盘里的东西不能拿出来
                  (bind _asbp_food_2 (Utilities|Casting|CastToBP_Food (Variables|Default|GetCurrentItem)))
                  (if (Variables|/Game/Blueprints/BP_Food.BP_Food_C|GetbCanPutInBowl _asbp_food_2)
                    (bind _asbp_bowl_2 (Utilities|Casting|CastToBP_Bowl (Variables|Default|GetCollisionActor))
                      (:then
                        (Development|PrintString "BOWLLLLLLLLLLLLLLLLLLLLLLLLLL")
                        (Default|GetFoodinBowl _asbp_bowl_2 _asbp_food_2 self)
                        (goto _label))
                      (:CastFailed
                        (goto _label_2)))
                    (else
                      (goto _label_2)))))))
          (else
            (bind _asbp_basket (Utilities|Casting|CastToBP_Basket _collisionactor)
              (:then
                (if (not (Variables|/Game/Blueprints/BP_Basket.BP_Basket_C|GetHasItem _asbp_basket))
                  (Default|SpawnGood _asbp_basket self)))
              (:CastFailed
                (bind _asbp_food_3 (Utilities|Casting|CastToBP_Food _collisionactor)
                  (:then
                    (if (not (Variables|/Game/Blueprints/BP_Food.BP_Food_C|GetbMustPutInBowl _asbp_food_3))
                      (if (not (Variables|/Game/Blueprints/BP_PickupItem.BP_PickupItem_C|GetbHolding _asbp_food_3))
                        (Default|PickUp2 _asbp_food_3 (Variables|Default|GetCookType)))))
                  (:CastFailed
                    (bind _asbp_pickup_item (Utilities|Casting|CastToBP_PickupItem _collisionactor)
                      (:then
                        (Default|PickUp2 _asbp_pickup_item (Variables|Default|GetCookType)))
                      (:CastFailed
                        (bind _asbp_cabinet (Utilities|Casting|CastToBP_Cabinet _collisionactor))
                        (Default|SpawnBowl _asbp_cabinet (Variables|Default|GetCookType))
                        (if (Utilities|Enum|Equal(Enum) (Variables|Default|GetCookType) "PLAYER")
                          _)))))))))))))

(event Input|ActionEvents|InputActionOperate
  (params (Key :type Key%20Structure :default "None")))

(event Input|ActionEvents|InputActionPickUpDrop
  (params (Key :type Key%20Structure :default "None"))
  ;[1 1 1] Record Player Tranjectories for Python data analysis
)

(event Input|ActionEvents|InputActionOperate
  (params (Key :type Key%20Structure :default "None"))
  ;[1 1 1] Record Player Tranjectories for Python data analysis
)

(event Input|ActionEvents|InputActionOperate
  (params (Key :type Key%20Structure :default "None"))
  (bind _currentcooktool (Variables|Default|GetCurrentCookTool))
  ;[1 1 1] Q Click: Operation
  (:Pressed
    (Variables|Default|SetTimeNoInput 0.0)
    (if (not (Variables|Default|GetbHoldingItem))
      (if (!= _currentcooktool 0)
        (bind _asbp_cutboard (Utilities|Casting|CastToBP_Cutboard _currentcooktool)
          (:then
            (Default|Cut _asbp_cutboard self))
          (:CastFailed
            (bind _asbp_cooker (Utilities|Casting|CastToBP_Cooker _currentcooktool)
              (:then
                (Default|FireCook _asbp_cooker self))
              (:CastFailed
                (bind _asbp_jucier (Utilities|Casting|CastToBP_Jucier _currentcooktool))
                (Default|MakeJuice _asbp_jucier self)
                (Class|TaskPawn|ClearAppleinJuicer (Variables|Default|GetMyTaskPawn))))))))))

(event Input|AxisEvents|InputAxisMoveForward
  (params (AxisValue :type Float%20%28single-precision%29))
  (bind _capsulecomponent (Variables|Collision|GetCapsuleComponent))
  ;[1 1 1] Movement
  (if (> AxisValue 0.0)
    (Variables|Default|SetTimeNoInput 0.0))
  (if (Variables|Default|GetbCanMove)
    (if (> AxisValue 0.0)
      (Transformation|SetWorldRotation _capsulecomponent "0, 0, 0" false true)
      (Pawn|Input|AddMovementInput "1.000000, 0, 0" AxisValue false :!label _label)
      (elif (< AxisValue 0.0)
        (Transformation|SetWorldRotation _capsulecomponent "0.000000,180.000000,0.000000" false true)
        (goto _label)))))

(event Input|AxisEvents|InputAxisMoveRight
  (params (AxisValue :type Float%20%28single-precision%29))
  (bind _capsulecomponent (Variables|Collision|GetCapsuleComponent))
  ;[1 1 1] Movement
  (if (> AxisValue 0.0)
    (Variables|Default|SetTimeNoInput 0.0))
  (if (Variables|Default|GetbCanMove)
    (if (> AxisValue 0.0)
      (Transformation|SetWorldRotation _capsulecomponent "0.000000,90.000000,0.000000" false true)
      (Pawn|Input|AddMovementInput "0.000000,1.000000, 0" AxisValue false :!label _label)
      (elif (< AxisValue 0.0)
        (Transformation|SetWorldRotation _capsulecomponent "0.000000,270.000000,0.000000" false true)
        (goto _label)))))

(event OnComponentBeginOverlap(Box)
  (params (OverlappedComponent :type Primitive%20Component%20Object%20Reference) (OtherActor :type Actor%20Object%20Reference) (OtherComp :type Primitive%20Component%20Object%20Reference) (OtherBodyIndex :type Integer) (bFromSweep :type Boolean) (SweepResult :type Hit%20Result%20Structure%20%28by%20ref%29))
  (bind _self self)
  ;[1 1 1] 碰撞结算顺序：物品 果篮 橱柜 空位 工具
  (bind _assimple_overcooked_game_mode (Utilities|Casting|CastToSimpleOvercookedGameMode (Game|GetGameMode)))
  (switch Utilities|FlowControl|Switch|SwitchonECOOKGAMEMODE (Variables|/Game/Blueprints/SimpleOvercookedGameMode.SimpleOvercookedGameMode_C|GetCookGameMode _assimple_overcooked_game_mode)
    (:IN_TURN
      (Utilities|FlowControl|Sequence
        (:then_0
          ;[1 1 1] Inspect
          (bind _asbp_inspect_tool (Utilities|Casting|CastToBP_InspectTool OtherActor :!label _label))
          (if (== (Variables|/Game/Blueprints/BP_InspectTool.BP_InspectTool_C|GetCookToolCollisionActor _asbp_inspect_tool) 0)
            (Variables|Default|SetCurrentCookTool _asbp_inspect_tool)
            (Variables|/Game/Blueprints/BP_InspectTool.BP_InspectTool_C|SetCookToolCollisionActor _asbp_inspect_tool _self)))
        (:then_1
          (if (== (Variables|Default|GetCollisionActor) 0)
            ;[1 1 1] Pickupdrop
            (bind _asbp_pickup_item (Utilities|Casting|CastToBP_PickupItem OtherActor :!label _label_2)
              (:then
                (Variables|Default|SetCollisionActor _asbp_pickup_item)
                (Variables|/Game/Blueprints/BP_PickupItem.BP_PickupItem_C|SetPickUpCollisionActor _asbp_pickup_item _self))
              (:CastFailed
                (bind _asbp_basket (Utilities|Casting|CastToBP_Basket OtherActor)
                  (:then
                    (Variables|Default|SetCollisionActor _asbp_basket)
                    (Variables|/Game/Blueprints/BP_Basket.BP_Basket_C|SetBasketCollisionActor _asbp_basket _self))
                  (:CastFailed
                    (bind _asbp_cabinet (Utilities|Casting|CastToBP_Cabinet OtherActor)
                      (:then
                        (Variables|Default|SetCollisionActor _asbp_cabinet)
                        (Variables|/Game/Blueprints/BP_Cabinet.BP_Cabinet_C|SetCabinetCollisionActor _asbp_cabinet _self))
                      (:CastFailed
                        (bind _asbp_trashbin (Utilities|Casting|CastToBP_Trashbin OtherActor)
                          (:then
                            (Variables|Default|SetCollisionActor _asbp_trashbin)
                            (Variables|/Game/Blueprints/BP_Trashbin.BP_Trashbin_C|SetTrashCollisionActor _asbp_trashbin _self))
                          (:CastFailed
                            (bind _asbp_cabinet_cup (Utilities|Casting|CastToBP_CabinetCup OtherActor))
                            (Variables|Default|SetCollisionActor _asbp_cabinet_cup)
                            (Variables|/Game/Blueprints/BP_CabinetCup.BP_CabinetCup_C|SetCabinetCollisionActor _asbp_cabinet_cup _self)))))))))))))
    (:TOGETHER
      (Utilities|FlowControl|Sequence
        (:then_0
          (goto _label))
        (:then_1
          (goto _label_2))))))

(event OnComponentEndOverlap(Box)
  (params (OverlappedComponent :type Primitive%20Component%20Object%20Reference) (OtherActor :type Actor%20Object%20Reference) (OtherComp :type Primitive%20Component%20Object%20Reference) (OtherBodyIndex :type Integer))
  (bind _asbp_pickup_item (Utilities|Casting|CastToBP_PickupItem OtherActor)
    (:then
      (Variables|/Game/Blueprints/BP_PickupItem.BP_PickupItem_C|SetPickUpCollisionActor _asbp_pickup_item 0)
      (Variables|Default|SetCollisionActor 0))
    (:CastFailed
      (bind _asbp_basket (Utilities|Casting|CastToBP_Basket OtherActor)
        (:then
          (Variables|/Game/Blueprints/BP_Basket.BP_Basket_C|SetBasketCollisionActor _asbp_basket 0)
          (Variables|Default|SetCollisionActor 0))
        (:CastFailed
          (bind _asbp_cabinet (Utilities|Casting|CastToBP_Cabinet OtherActor)
            (:then
              (Variables|/Game/Blueprints/BP_Cabinet.BP_Cabinet_C|SetCabinetCollisionActor _asbp_cabinet 0)
              (Variables|Default|SetCollisionActor 0))
            (:CastFailed
              (bind _asbp_trashbin (Utilities|Casting|CastToBP_Trashbin OtherActor))
              (Variables|/Game/Blueprints/BP_Trashbin.BP_Trashbin_C|SetTrashCollisionActor _asbp_trashbin 0)
              (Variables|Default|SetCollisionActor 0))))))))

(event Custom|CustomEvent
  (params (OverlappedComponent :type Primitive%20Component%20Object%20Reference) (OtherActor :type Actor%20Object%20Reference) (OtherComp :type Primitive%20Component%20Object%20Reference) (OtherBodyIndex :type Integer)))

(fn ConstructionScript)

(fn CheckCurrentHoldingItem
  (bind _currentitem (Variables|Default|GetCurrentItem))
  (if (!= _currentitem 0)
    (bind _returnvalue (Class|TaskPawn|GetPlannableNameforAI (Variables|Default|GetMyTaskPawn) (Utilities|GetDisplayName _currentitem)))
    (return _returnvalue)))