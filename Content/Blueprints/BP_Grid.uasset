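; BP_Grid is a placement slot actor that snaps and holds a single BP_PickupItem.
; When an item that is neither held nor already gridded begins overlapping its Box, the free slot stops physics, teleports the item to its transform, marks both occupied and optionally hides the mesh.
; Tick frees the slot once the item is held or off-grid.
; End-overlap release attempts remain as unconnected, never-run logic.
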(event OnActorEndOverlap(OccupiedItem)
  (params (OverlappedActor :type Actor%20Object%20Reference) (OtherActor :type Actor%20Object%20Reference))
  ;[0 0.601 0.277 0.345] Delete
)

(event OnComponentBeginOverlap(Box)
  (params (OverlappedComponent :type Primitive%20Component%20Object%20Reference) (OtherActor :type Actor%20Object%20Reference) (OtherComp :type Primitive%20Component%20Object%20Reference) (OtherBodyIndex :type Integer) (bFromSweep :type Boolean) (SweepResult :type Hit%20Result%20Structure%20%28by%20ref%29))
  (if (not (Variables|Default|GetbOccupied))
    (bind _asbp_pickup_item (Utilities|Casting|CastToBP_PickupItem OtherActor))
    (if (not (Variables|/Game/Blueprints/BP_PickupItem.BP_PickupItem_C|GetbHolding _asbp_pickup_item))
      (if (not (Variables|/Game/Blueprints/BP_PickupItem.BP_PickupItem_C|GetbOnGrid _asbp_pickup_item))
        (Physics|SetSimulatePhysics (Variables|/Game/Blueprints/BP_PickupItem.BP_PickupItem_C|GetStaticMesh _asbp_pickup_item) false)
        (Collision|SetCollisionEnabled (Variables|/Game/Blueprints/BP_PickupItem.BP_PickupItem_C|GetStaticMesh _asbp_pickup_item) "NoCollision")
        (Transformation|SetActorLocation _asbp_pickup_item (Transformation|GetActorLocation) false true)
        (Transformation|SetActorRotation _asbp_pickup_item (Transformation|GetActorRotation) true)
        (Variables|Default|SetbOccupied true)
        (Variables|/Game/Blueprints/BP_PickupItem.BP_PickupItem_C|SetbOnGrid _asbp_pickup_item true)
        (Variables|Default|SetOccupiedItem _asbp_pickup_item)
        (Collision|SetCollisionEnabled (Variables|/Game/Blueprints/BP_PickupItem.BP_PickupItem_C|GetStaticMesh _asbp_pickup_item) "QueryAndPhysics")
        (if (Variables|Default|GetbItemInVisible)
          (Rendering|SetVisibility (Variables|/Game/Blueprints/BP_PickupItem.BP_PickupItem_C|GetStaticMesh _asbp_pickup_item) false false))))))

(event OnComponentEndOverlap(Box)
  (params (OverlappedComponent :type Primitive%20Component%20Object%20Reference) (OtherActor :type Actor%20Object%20Reference) (OtherComp :type Primitive%20Component%20Object%20Reference) (OtherBodyIndex :type Integer))
  ;[0 0.601 0.277 0.345] Delete
)

(event EventBeginPlay)

(event Collision|EventActorBeginOverlap
  (params (OtherActor :type Actor%20Object%20Reference)))

(event EventTick
  (params (DeltaSeconds :type Float%20%28single-precision%29))
  (if (!= (Variables|Default|GetOccupiedItem) 0)
    (if (or (Variables|/Game/Blueprints/BP_PickupItem.BP_PickupItem_C|GetbHolding (Variables|Default|GetOccupiedItem)) (not (Variables|/Game/Blueprints/BP_PickupItem.BP_PickupItem_C|GetbOnGrid (Variables|Default|GetOccupiedItem))))
      (Variables|Default|SetOccupiedItem 0)
      (Variables|Default|SetbOccupied false))))

(fn ConstructionScript)