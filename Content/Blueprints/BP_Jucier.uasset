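; BP_Jucier is a juicer station that captures food dropped into its box and is meant to turn it into juice.
; Overlapping BP_Food that is unheld, off-grid and juicer-eligible snaps to the actor and joins OwnedFood.
; MakeJuice only fetches the progress widget; the timeline that fills the bar and then flags the first food for a bowl, re-skinning Green Apple, is disconnected and never runs.
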(event OnComponentBeginOverlap(Box)
  (params (OverlappedComponent :type Primitive%20Component%20Object%20Reference) (OtherActor :type Actor%20Object%20Reference) (OtherComp :type Primitive%20Component%20Object%20Reference) (OtherBodyIndex :type Integer) (bFromSweep :type Boolean) (SweepResult :type Hit%20Result%20Structure%20%28by%20ref%29))
  (bind _asbp_food (Utilities|Casting|CastToBP_Food OtherActor))
  ;[1 1 1] Condition: not holding, not on grid, can be put in juicer
  (if (not (Variables|/Game/Blueprints/BP_PickupItem.BP_PickupItem_C|GetbHolding _asbp_food))
    (if (not (Variables|/Game/Blueprints/BP_PickupItem.BP_PickupItem_C|GetbOnGrid _asbp_food))
      (if (Variables|/Game/Blueprints/BP_Food.BP_Food_C|GetbCanPutInJuicer _asbp_food)
        (Collision|SetCollisionEnabled (Variables|/Game/Blueprints/BP_PickupItem.BP_PickupItem_C|GetStaticMesh _asbp_food) "NoCollision")
        (Physics|SetSimulatePhysics (Variables|/Game/Blueprints/BP_PickupItem.BP_PickupItem_C|GetStaticMesh _asbp_food) false)
        (Transformation|SetActorLocation _asbp_food (Transformation|GetActorLocation) false false)
        (Variables|/Game/Blueprints/BP_PickupItem.BP_PickupItem_C|SetbOnGrid _asbp_food true)
        (Collision|SetCollisionEnabled (Variables|/Game/Blueprints/BP_PickupItem.BP_PickupItem_C|GetStaticMesh _asbp_food) "QueryAndPhysics")
        (Rendering|SetVisibility (Variables|/Game/Blueprints/BP_PickupItem.BP_PickupItem_C|GetStaticMesh _asbp_food) true false)
        (Utilities|Array|Add (Variables|Default|GetOwnedFood) _asbp_food)))))

(event Custom|MakeJuice
  (params (who :type BP%20Cook%20Object%20Reference))
  (if (!= (Utilities|Array|Length (Variables|Default|GetOwnedFood)) 0)
    ;[1 1 1] NO LINK!!!!!!!!!!!!!!!!!!!!!
    (bind _asprogress_bar_widget (Utilities|Casting|CastToProgressBarWidget (UserInterface|GetUserWidgetObject (Variables|Default|GetProgressWidgetComp))))))

(event EventBeginPlay)

(event Collision|EventActorBeginOverlap
  (params (OtherActor :type Actor%20Object%20Reference)))

(event EventTick
  (params (DeltaSeconds :type Float%20%28single-precision%29)))

(fn ConstructionScript)