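; Pickup item that cooks can hold and drop, tracking its state as an abstract location.
; PickUp2 attaches it to the overlapping BP_Cook's HoldComponent if the cook type matches, disabling physics and updating both item and cook state.
; Drop detaches it, restores physics and collision, pushes it forward by mass-scaled force, and reports an unknown location to the player cook's task pawn.
; The event graph holds only empty or unreachable logic.
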(event EventBeginPlay)

(event Collision|EventActorBeginOverlap
  (params (OtherActor :type Actor%20Object%20Reference)))

(event EventTick
  (params (DeltaSeconds :type Float%20%28single-precision%29)))

(event Collision|EventActorEndOverlap
  (params (OtherActor :type Actor%20Object%20Reference))
  ;[0.4774 1 0.3175] ~Delete Collision End Overlap Handled in BP_Cook
)

(fn ConstructionScript)

(fn PickUp2
  (params (NewParam :type ECOOKTYPE%20Enum :default "PLAYER"))
  (bind _staticmesh (Variables|Default|GetStaticMesh))
  (Physics|SetSimulatePhysics _staticmesh false)
  (bind _asbp_cook (Utilities|Casting|CastToBP_Cook (Variables|Default|GetPickUpCollisionActor)))
  (if (Utilities|Enum|Equal(Enum) (Variables|/Game/Blueprints/BP_Cook.BP_Cook_C|GetCookType _asbp_cook) NewParam)
    (Transformation|AttachComponentToComponent (Variables|/Game/Blueprints/BP_Cook.BP_Cook_C|GetHoldComponent _asbp_cook) "None" "SnapToTarget" "SnapToTarget" "KeepWorld" false)
    (Collision|SetCollisionEnabled _staticmesh "NoCollision")
    (Variables|/Game/Blueprints/BP_Cook.BP_Cook_C|SetCurrentItem _asbp_cook self)
    (Variables|/Game/Blueprints/BP_Cook.BP_Cook_C|SetbHoldingItem _asbp_cook true)
    (Variables|Default|SetbOnGrid false)
    (Variables|Default|SetbHolding true)
    (Variables|Default|SetAbstractLocation "BE_HOLD")
    (if (Variables|/Script/Engine.SceneComponent|GetbVisible _staticmesh)
      _
      (else
        (Rendering|SetVisibility _staticmesh true false)
        (Collision|SetCollisionEnabled _staticmesh "QueryOnly")))
    (bind _asbp_cook_2 (Utilities|Casting|CastToBP_Cook (Game|GetPlayerCharacter 0)))))

(fn Drop
  (params (itemn :type String) (type :type ECOOKTYPE%20Enum :default "PLAYER"))
  (bind _staticmesh (Variables|Default|GetStaticMesh))
  (Variables|Default|SetbHolding false)
  (Physics|SetSimulatePhysics _staticmesh true)
  (Collision|SetCollisionEnabled _staticmesh "PhysicsOnly")
  (Transformation|DetachFromComponent _staticmesh "KeepWorld" "KeepWorld" "KeepRelative" true)
  (bind _asbp_cook (Utilities|Casting|CastToBP_Cook (Game|GetPlayerCharacter 0)))
  (Class|TaskPawn|ChangeItemAbstractLocation (Variables|/Game/Blueprints/BP_Cook.BP_Cook_C|GetMyTaskPawn _asbp_cook) itemn "UNKNOWN")
  (Physics|AddForce _staticmesh (* (Math|Vector|GetForwardVector _staticmesh) (* (Physics|GetMass (Variables|Default|GetStaticMesh)) 1e+04)) "None" false)
  (Collision|SetCollisionEnabled _staticmesh "QueryAndPhysics")
  (Variables|Default|SetAbstractLocation "UNKNOWN")
  (return true))