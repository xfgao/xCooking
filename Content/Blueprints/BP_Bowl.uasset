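; BP_Bowl is a cooking-game bowl that collects ingredients and turns them into a hamburger.
; GetFoodInBowl attaches food to ContainComp with physics off, updates the player cook's task pawn, then calls ShowFoodUI.
; ShowFoodUI removes held ingredients from the Burger recipe array and shows their sprites on the BowlItemUI widget.
; Once Burger is empty, it hides each held ingredient and spawns an attached hamburger-mesh BP_Food per ingredient.
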(event Custom|ShowFoodUI
  (bind _self self)
  (bind _burger (Variables|Default|GetBurger))
  (bind _bowlholdactors (Variables|Default|GetBowlHoldActors))
  (bind _rootcomponent (Variables|/Script/Engine.Actor|GetRootComponent _self))
  (bind _returnvalue (Transformation|GetWorldTransform _rootcomponent))
  (bind (_location _rotation) (Math|Transform|BreakTransform _returnvalue))
  (bind _asbowl_item_ui (Utilities|Casting|CastToBowlItemUI (UserInterface|GetUserWidgetObject (Variables|Default|GetWidget))))
  (Variables|Default|Setitems 0)
  (for _index (range 0 (- (Utilities|Array|Length _bowlholdactors) 1))
    (if (!= (Utilities|Array|FindItem _burger (Variables|/Game/Blueprints/BP_Food.BP_Food_C|GetFoodName (Utilities|Array|Get(acopy) _bowlholdactors _index))) -1)
      (Utilities|Array|RemoveIndex _burger (Utilities|Array|FindItem _burger (Variables|/Game/Blueprints/BP_Food.BP_Food_C|GetFoodName (Utilities|Array|Get(acopy) _bowlholdactors _index))))
      (switch Utilities|FlowControl|Switch|SwitchonFoodList (Variables|/Game/Blueprints/BP_Food.BP_Food_C|GetFoodName (Utilities|Array|Get(acopy) _bowlholdactors _index))
        (:NewEnumerator1
          (Development|PrintString "Hello Green Apple"))
        (:NewEnumerator4
          (Class|Image|SetBrush (Utilities|Array|Get(acopy) (Variables|/Game/Blueprints/kitchen4/BowlItemUI.BowlItemUI_C|GetImage_Array _asbowl_item_ui) _index) (Utilities|Struct|MakeSlateBrush (.ImageSize (Utilities|Struct|BreakSlateBrush (Variables|/Script/UMG.Image|GetBrush (Utilities|Array|Get(acopy) (Variables|/Game/Blueprints/kitchen4/BowlItemUI.BowlItemUI_C|GetImage_Array _asbowl_item_ui) _index)))) (.Margin (Utilities|Struct|BreakSlateBrush (Variables|/Script/UMG.Image|GetBrush (Utilities|Array|Get(acopy) (Variables|/Game/Blueprints/kitchen4/BowlItemUI.BowlItemUI_C|GetImage_Array _asbowl_item_ui) _index)))) (.TintColor (Utilities|Struct|BreakSlateBrush (Variables|/Script/UMG.Image|GetBrush (Utilities|Array|Get(acopy) (Variables|/Game/Blueprints/kitchen4/BowlItemUI.BowlItemUI_C|GetImage_Array _asbowl_item_ui) _index)))) "/Game/Blueprints/kitchen4/Tomato_Sprite.Tomato_Sprite" (.DrawAs (Utilities|Struct|BreakSlateBrush (Variables|/Script/UMG.Image|GetBrush (Utilities|Array|Get(acopy) (Variables|/Game/Blueprints/kitchen4/BowlItemUI.BowlItemUI_C|GetImage_Array _asbowl_item_ui) _index)))) (.Tiling (Utilities|Struct|BreakSlateBrush (Variables|/Script/UMG.Image|GetBrush (Utilities|Array|Get(acopy) (Variables|/Game/Blueprints/kitchen4/BowlItemUI.BowlItemUI_C|GetImage_Array _asbowl_item_ui) _index)))) (.Mirroring (Utilities|Struct|BreakSlateBrush (Variables|/Script/UMG.Image|GetBrush (Utilities|Array|Get(acopy) (Variables|/Game/Blueprints/kitchen4/BowlItemUI.BowlItemUI_C|GetImage_Array _asbowl_item_ui) _index))))))
          (Widget|SetVisibility (Utilities|Array|Get(acopy) (Variables|/Game/Blueprints/kitchen4/BowlItemUI.BowlItemUI_C|GetImage_Array _asbowl_item_ui) _index) "Visible" :!label _label))
        (:NewEnumerator5
          (Class|Image|SetBrush (Utilities|Array|Get(acopy) (Variables|/Game/Blueprints/kitchen4/BowlItemUI.BowlItemUI_C|GetImage_Array _asbowl_item_ui) _index) (Utilities|Struct|MakeSlateBrush (.ImageSize (Utilities|Struct|BreakSlateBrush (Variables|/Script/UMG.Image|GetBrush (Utilities|Array|Get(acopy) (Variables|/Game/Blueprints/kitchen4/BowlItemUI.BowlItemUI_C|GetImage_Array _asbowl_item_ui) _index)))) (.Margin (Utilities|Struct|BreakSlateBrush (Variables|/Script/UMG.Image|GetBrush (Utilities|Array|Get(acopy) (Variables|/Game/Blueprints/kitchen4/BowlItemUI.BowlItemUI_C|GetImage_Array _asbowl_item_ui) _index)))) (.TintColor (Utilities|Struct|BreakSlateBrush (Variables|/Script/UMG.Image|GetBrush (Utilities|Array|Get(acopy) (Variables|/Game/Blueprints/kitchen4/BowlItemUI.BowlItemUI_C|GetImage_Array _asbowl_item_ui) _index)))) "/Game/Blueprints/kitchen4/Meat_Sprite.Meat_Sprite" (.DrawAs (Utilities|Struct|BreakSlateBrush (Variables|/Script/UMG.Image|GetBrush (Utilities|Array|Get(acopy) (Variables|/Game/Blueprints/kitchen4/BowlItemUI.BowlItemUI_C|GetImage_Array _asbowl_item_ui) _index)))) (.Tiling (Utilities|Struct|BreakSlateBrush (Variables|/Script/UMG.Image|GetBrush (Utilities|Array|Get(acopy) (Variables|/Game/Blueprints/kitchen4/BowlItemUI.BowlItemUI_C|GetImage_Array _asbowl_item_ui) _index)))) (.Mirroring (Utilities|Struct|BreakSlateBrush (Variables|/Script/UMG.Image|GetBrush (Utilities|Array|Get(acopy) (Variables|/Game/Blueprints/kitchen4/BowlItemUI.BowlItemUI_C|GetImage_Array _asbowl_item_ui) _index))))))
          (goto _label))
        (:NewEnumerator6
          (Class|Image|SetBrush (Utilities|Array|Get(acopy) (Variables|/Game/Blueprints/kitchen4/BowlItemUI.BowlItemUI_C|GetImage_Array _asbowl_item_ui) _index) (Utilities|Struct|MakeSlateBrush (.ImageSize (Utilities|Struct|BreakSlateBrush (Variables|/Script/UMG.Image|GetBrush (Utilities|Array|Get(acopy) (Variables|/Game/Blueprints/kitchen4/BowlItemUI.BowlItemUI_C|GetImage_Array _asbowl_item_ui) _index)))) (.Margin (Utilities|Struct|BreakSlateBrush (Variables|/Script/UMG.Image|GetBrush (Utilities|Array|Get(acopy) (Variables|/Game/Blueprints/kitchen4/BowlItemUI.BowlItemUI_C|GetImage_Array _asbowl_item_ui) _index)))) (.TintColor (Utilities|Struct|BreakSlateBrush (Variables|/Script/UMG.Image|GetBrush (Utilities|Array|Get(acopy) (Variables|/Game/Blueprints/kitchen4/BowlItemUI.BowlItemUI_C|GetImage_Array _asbowl_item_ui) _index)))) "/Game/Blueprints/kitchen4/Lettuce_Sprite.Lettuce_Sprite" (.DrawAs (Utilities|Struct|BreakSlateBrush (Variables|/Script/UMG.Image|GetBrush (Utilities|Array|Get(acopy) (Variables|/Game/Blueprints/kitchen4/BowlItemUI.BowlItemUI_C|GetImage_Array _asbowl_item_ui) _index)))) (.Tiling (Utilities|Struct|BreakSlateBrush (Variables|/Script/UMG.Image|GetBrush (Utilities|Array|Get(acopy) (Variables|/Game/Blueprints/kitchen4/BowlItemUI.BowlItemUI_C|GetImage_Array _asbowl_item_ui) _index)))) (.Mirroring (Utilities|Struct|BreakSlateBrush (Variables|/Script/UMG.Image|GetBrush (Utilities|Array|Get(acopy) (Variables|/Game/Blueprints/kitchen4/BowlItemUI.BowlItemUI_C|GetImage_Array _asbowl_item_ui) _index))))))
          (goto _label))
        (:NewEnumerator7
          (Class|Image|SetBrush (Utilities|Array|Get(acopy) (Variables|/Game/Blueprints/kitchen4/BowlItemUI.BowlItemUI_C|GetImage_Array _asbowl_item_ui) _index) (Utilities|Struct|MakeSlateBrush (.ImageSize (Utilities|Struct|BreakSlateBrush (Variables|/Script/UMG.Image|GetBrush (Utilities|Array|Get(acopy) (Variables|/Game/Blueprints/kitchen4/BowlItemUI.BowlItemUI_C|GetImage_Array _asbowl_item_ui) _index)))) (.Margin (Utilities|Struct|BreakSlateBrush (Variables|/Script/UMG.Image|GetBrush (Utilities|Array|Get(acopy) (Variables|/Game/Blueprints/kitchen4/BowlItemUI.BowlItemUI_C|GetImage_Array _asbowl_item_ui) _index)))) (.TintColor (Utilities|Struct|BreakSlateBrush (Variables|/Script/UMG.Image|GetBrush (Utilities|Array|Get(acopy) (Variables|/Game/Blueprints/kitchen4/BowlItemUI.BowlItemUI_C|GetImage_Array _asbowl_item_ui) _index)))) "/Game/Blueprints/kitchen4/Bread_Sprite.Bread_Sprite" (.DrawAs (Utilities|Struct|BreakSlateBrush (Variables|/Script/UMG.Image|GetBrush (Utilities|Array|Get(acopy) (Variables|/Game/Blueprints/kitchen4/BowlItemUI.BowlItemUI_C|GetImage_Array _asbowl_item_ui) _index)))) (.Tiling (Utilities|Struct|BreakSlateBrush (Variables|/Script/UMG.Image|GetBrush (Utilities|Array|Get(acopy) (Variables|/Game/Blueprints/kitchen4/BowlItemUI.BowlItemUI_C|GetImage_Array _asbowl_item_ui) _index)))) (.Mirroring (Utilities|Struct|BreakSlateBrush (Variables|/Script/UMG.Image|GetBrush (Utilities|Array|Get(acopy) (Variables|/Game/Blueprints/kitchen4/BowlItemUI.BowlItemUI_C|GetImage_Array _asbowl_item_ui) _index))))))
          (goto _label)))))
  (Widget|SetVisibility (Variables|/Game/Blueprints/kitchen4/BowlItemUI.BowlItemUI_C|GetImage_358 _asbowl_item_ui) "Visible")
  (if (== (Utilities|Array|Length (Variables|Default|GetBurger)) 0)
    (for _array_element (Variables|Default|GetBowlHoldActors)
      (Rendering|SetVisibility (Variables|/Game/Blueprints/BP_PickupItem.BP_PickupItem_C|GetStaticMesh _array_element) false true)
      (bind _returnvalue_2 (Game|SpawnActorfromClass "/Game/Blueprints/BP_Food.BP_Food_C" (Math|Transform|MakeTransform _location _rotation "0.300000,0.300000,0.300000") "Undefined" 0 0))
      (Components|StaticMesh|SetStaticMesh (Variables|/Game/Blueprints/BP_PickupItem.BP_PickupItem_C|GetStaticMesh _returnvalue_2) "/Game/Assets/food/hamburgeres.hamburgeres")
      (Physics|SetSimulatePhysics (Variables|/Game/Blueprints/BP_PickupItem.BP_PickupItem_C|GetStaticMesh _returnvalue_2) false)
      (Collision|SetCollisionEnabled (Variables|/Game/Blueprints/BP_PickupItem.BP_PickupItem_C|GetStaticMesh _returnvalue_2) "NoCollision")
      (Transformation|AttachComponentToComponent (Variables|/Game/Blueprints/BP_PickupItem.BP_PickupItem_C|GetStaticMesh _returnvalue_2) (Variables|Default|GetContainComp) "None" "SnapToTarget" "KeepRelative" "KeepWorld" true))))

(event EventBeginPlay)

(event Collision|EventActorBeginOverlap
  (params (OtherActor :type Actor%20Object%20Reference)))

(fn ConstructionScript)

(fn DropBowl
  ;[0.2719 1 0.1332] ~Delete
)

(fn GetFoodinBowl
  (params (food :type BP%20Food%20Object%20Reference) (who :type BP%20Cook%20Object%20Reference))
  (bind _returnvalue (Utilities|GetDisplayName food))
  (bind _staticmesh (Variables|/Game/Blueprints/BP_PickupItem.BP_PickupItem_C|GetStaticMesh food))
  (bind _containcomp (Variables|Default|GetContainComp))
  (Utilities|FlowControl|Sequence
    (:then_0
      ;[1 1 1] AttachFood to Bowl
      (Utilities|FlowControl|Sequence
        (:then_0
          (Utilities|Array|Add (Variables|Default|GetBowlHoldActors) food)
          (Variables|/Game/Blueprints/BP_PickupItem.BP_PickupItem_C|SetbHolding food true)
          (Transformation|DetachFromComponent _staticmesh "KeepWorld" "KeepWorld" "KeepRelative" true)
          (Rendering|SetVisibility _staticmesh true false)
          (Physics|SetSimulatePhysics _staticmesh false)
          (Collision|SetCollisionEnabled _staticmesh "NoCollision")
          (Transformation|AttachComponentToComponent _staticmesh _containcomp "None" "SnapToTarget" "KeepRelative" "KeepRelative" true)
          (Transformation|AddRelativeRotation _containcomp (Math|Rotator|MakeRotator 0.0 0.0 (* 0 4e+01)) false false)
          (Variables|Default|SetitemNum (+ (Variables|Default|GetitemNum) 1)))
        (:then_1
          (bind _asbp_cook (Utilities|Casting|CastToBP_Cook (Game|GetPlayerCharacter 0)))
          ;[1 1 1] Cpp
          (Class|TaskPawn|AddKitchenItemAttribute (Variables|/Game/Blueprints/BP_Cook.BP_Cook_C|GetMyTaskPawn _asbp_cook) (Utilities|GetDisplayName self) _returnvalue (Variables|/Game/Blueprints/BP_Cook.BP_Cook_C|GetCookType who))
          (Class|TaskPawn|DeleteKitchenIteminLevelItems (Variables|/Game/Blueprints/BP_Cook.BP_Cook_C|GetMyTaskPawn _asbp_cook) _returnvalue))))
    (:then_1
      (CallFunction|ShowFoodUI))))