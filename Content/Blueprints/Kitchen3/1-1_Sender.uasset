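; Order delivery station for an Overcooked-style kitchen level that takes and judges the cook's held item.
; Dump destroys that item and any bowl contents, removing it from the task pawn's level items.
; CheckSuccess checks its name against the required task item, plays success or fail UI animation, and on success increments the order count and adds a hard-coded Green Apple Juice task.
; An HTTP stats upload sits unconnected.
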(event Custom|Dump
  (bind _asbp_cook (Utilities|Casting|CastToBP_Cook (Variables|Default|GetTrashCollisionActor)))
  (bind _asbp_bowl (Utilities|Casting|CastToBP_Bowl (Variables|/Game/Blueprints/BP_Cook.BP_Cook_C|GetCurrentItem _asbp_cook))
    (:then
      (for _array_element (Variables|/Game/Blueprints/BP_Bowl.BP_Bowl_C|GetBowlHoldActors _asbp_bowl)
        (Actor|DestroyActor _array_element)))
    (:CastFailed
      _))
  (CallFunction|CheckSuccess (Variables|/Game/Blueprints/BP_Cook.BP_Cook_C|GetCurrentItem _asbp_cook))
  (Class|TaskPawn|DeleteKitchenIteminLevelItems (Variables|/Game/Blueprints/BP_Cook.BP_Cook_C|GetMyTaskPawn _asbp_cook) (Utilities|GetDisplayName (Variables|/Game/Blueprints/BP_Cook.BP_Cook_C|GetCurrentItem _asbp_cook)))
  (Actor|DestroyActor (Variables|/Game/Blueprints/BP_Cook.BP_Cook_C|GetCurrentItem _asbp_cook)))

(event Custom|CheckSuccess
  (params (Item :type BP%20Pickup%20Item%20Object%20Reference))
  (bind _asbp_cook (Utilities|Casting|CastToBP_Cook (Game|GetPlayerCharacter 0)))
  (Development|PrintString "Hello")
  (bind _returnvalue (Class|TaskPawn|CheckKitchenItembyName (Variables|/Game/Blueprints/BP_Cook.BP_Cook_C|GetMyTaskPawn _asbp_cook) (Utilities|GetDisplayName Item) (Variables|Default|GetTaskRequiredItem)))
  (bind _assuccess_fail (Utilities|Casting|CastToSuccessFail (UserInterface|GetUserWidgetObject (Variables|Default|GetWidget))))
  (if _returnvalue
    (Default|PlaySuccessAnimation _assuccess_fail)
    (Class|TaskPawn|DeleteKitchenIteminLevelItems (Variables|/Game/Blueprints/BP_Cook.BP_Cook_C|GetMyTaskPawn _asbp_cook) (Utilities|GetDisplayName (Variables|/Game/Blueprints/BP_Cook.BP_Cook_C|GetCurrentItem _asbp_cook)))
    (bind _assimple_overcooked_game_mode (Utilities|Casting|CastToSimpleOvercookedGameMode (Game|GetGameMode)))
    (Variables|/Game/Blueprints/SimpleOvercookedGameMode.SimpleOvercookedGameMode_C|SetGameSuccessfulOrder _assimple_overcooked_game_mode (+ (Variables|/Game/Blueprints/SimpleOvercookedGameMode.SimpleOvercookedGameMode_C|GetGameSuccessfulOrder _assimple_overcooked_game_mode) 1))
    (Class|TaskPawn|AddTaskTree (Variables|/Game/Blueprints/BP_Cook.BP_Cook_C|GetMyTaskPawn _asbp_cook) "Green Apple Juice")
    (else
      (Default|PlayFailAnimation _assuccess_fail))))

(fn ConstructionScript)