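; Juicer station for Kitchen 1-1 that turns three green apples into juice.
; Box overlap absorbs and destroys loose apples while updating the instruction widget's count display.
; MakeJuice runs a Timeline progress bar, then spawns a hidden BP_Food juice that must go in a bowl and marks the juicer occupied.
; Tick frees the juicer once that juice is held, and each stage updates kitchen item state on the cook's MyTaskPawn.
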(event OnComponentBeginOverlap(Box)
  (params (OverlappedComponent :type Primitive%20Component%20Object%20Reference) (OtherActor :type Actor%20Object%20Reference) (OtherComp :type Primitive%20Component%20Object%20Reference) (OtherBodyIndex :type Integer) (bFromSweep :type Boolean) (SweepResult :type Hit%20Result%20Structure%20%28by%20ref%29))
  ;[1 1 1] Collision Control
  (if (not (Variables|Default|GetbOccupied))
    (bind _asbp_food (Utilities|Casting|CastToBP_Food OtherActor))
    ;[1 1 1] Condition: not holding, not on grid, can be put in juicer
    (if (not (Variables|/Game/Blueprints/BP_PickupItem.BP_PickupItem_C|GetbHolding _asbp_food))
      (if (not (Variables|/Game/Blueprints/BP_PickupItem.BP_PickupItem_C|GetbOnGrid _asbp_food))
        (if (Variables|/Game/Blueprints/BP_Food.BP_Food_C|GetbCanPutInJuicer _asbp_food)
          (if (Utilities|Enum|Equal(Enum) (Variables|/Game/Blueprints/BP_Food.BP_Food_C|GetFoodName _asbp_food) "NewEnumerator1")
            (if (<= (Variables|Default|GetGreenAppleCount) 2)
              (Physics|SetSimulatePhysics (Variables|/Game/Blueprints/BP_PickupItem.BP_PickupItem_C|GetStaticMesh _asbp_food) false)
              (Collision|SetCollisionEnabled (Variables|/Game/Blueprints/BP_PickupItem.BP_PickupItem_C|GetStaticMesh _asbp_food) "NoCollision")
              (Transformation|SetActorLocation _asbp_food (Transformation|GetActorLocation) false false)
              (Variables|/Game/Blueprints/BP_PickupItem.BP_PickupItem_C|SetbOnGrid _asbp_food true)
              (Rendering|SetVisibility (Variables|/Game/Blueprints/BP_PickupItem.BP_PickupItem_C|GetStaticMesh _asbp_food) false false)
              (Variables|Default|SetGreenAppleCount (+ (Variables|Default|GetGreenAppleCount) 1))
              ;[1 1 1] Apple in Juicer cannot be picked up
              (Variables|/Game/Blueprints/BP_PickupItem.BP_PickupItem_C|SetbHolding _asbp_food true)
              (CallFunction|InstrunctionUISetting)
              ;[1 1 1] CPP: cook type is undefined
              (bind _asbp_cook (Utilities|Casting|CastToBP_Cook (Game|GetPlayerCharacter 0)))
              (Class|TaskPawn|AddKitchenItemAttribute (Variables|/Game/Blueprints/BP_Cook.BP_Cook_C|GetMyTaskPawn _asbp_cook) "Juicer Container" (Utilities|GetDisplayName _asbp_food) "PLAYER")
              (bind _asbp_cook_2 (Utilities|Casting|CastToBP_Cook (Game|GetPlayerCharacter 0)))
              (Class|TaskPawn|ChangeItemAbstractLocation (Variables|/Game/Blueprints/BP_Cook.BP_Cook_C|GetMyTaskPawn _asbp_cook_2) (Utilities|GetDisplayName OtherActor) "IN_JUCIER")
              (Actor|DestroyActor _asbp_food))))))))

(event Custom|MakeJuice
  (params (who :type BP%20Cook%20Object%20Reference))
  (bind _ownedfood (Variables|Default|GetOwnedFood))
  (bind _mytaskpawn (Variables|/Game/Blueprints/BP_Cook.BP_Cook_C|GetMyTaskPawn who))
  (bind _cooktype (Variables|/Game/Blueprints/BP_Cook.BP_Cook_C|GetCookType who))
  (bind _progresswidgetcomp (Variables|Default|GetProgressWidgetComp))
  ;[1 1 1] Make Juice
  (if (== (Variables|Default|GetGreenAppleCount) 3)
    (bind _asprogress_bar_widget (Utilities|Casting|CastToProgressBarWidget (UserInterface|GetUserWidgetObject _progresswidgetcomp)))
    (Rendering|SetVisibility _progresswidgetcomp true false)
    (bind _progress (Timeline|Timeline_Make_Juice PlayFromStart)
      (:Update
        (Progress|SetPercent (Variables|/Game/Blueprints/UI/ProgressBarWidget.ProgressBarWidget_C|GetProgressBar_53 _asprogress_bar_widget) _progress))
      (:Finished
        (Rendering|SetVisibility _progresswidgetcomp false false)
        (Utilities|FlowControl|Sequence
          (:then_0
            ;[1 1 1] New  Item
            (bind _returnvalue (Game|SpawnActorfromClass "/Game/Blueprints/BP_Food.BP_Food_C" (Transformation|GetActorTransform) "Undefined" 0 0))
            (Variables|/Game/Blueprints/BP_Food.BP_Food_C|SetbMustPutInBowl _returnvalue true)
            (Variables|/Game/Blueprints/BP_Food.BP_Food_C|SetbCanPutInBowl _returnvalue true)
            (Components|StaticMesh|SetStaticMesh (Variables|/Game/Blueprints/BP_PickupItem.BP_PickupItem_C|GetStaticMesh _returnvalue) "/Game/Assets/furniture/half2.half2")
            (Transformation|SetRelativeScale3D (Variables|/Game/Blueprints/BP_PickupItem.BP_PickupItem_C|GetStaticMesh _returnvalue) "0.800000,0.800000,0.800000")
            (Rendering|Material|SetMaterial (Variables|/Game/Blueprints/BP_PickupItem.BP_PickupItem_C|GetStaticMesh _returnvalue) 0 "/Game/Assets/food/apple_green/M_apple_G.M_apple_G")
            (Collision|SetCollisionEnabled (Variables|/Game/Blueprints/BP_PickupItem.BP_PickupItem_C|GetStaticMesh _returnvalue) "QueryAndPhysics")
            (Physics|SetSimulatePhysics (Variables|/Game/Blueprints/BP_PickupItem.BP_PickupItem_C|GetStaticMesh _returnvalue) false)
            (Rendering|SetVisibility (Variables|/Game/Blueprints/BP_PickupItem.BP_PickupItem_C|GetStaticMesh _returnvalue) false false)
            (Variables|/Game/Blueprints/BP_PickupItem.BP_PickupItem_C|SetAbstractLocation _returnvalue "BE_HOLD"))
          (:then_1
            (for _array_element (Variables|Default|GetOwnedFood)
              (bind _asbp_cook (Utilities|Casting|CastToBP_Cook (Game|GetPlayerCharacter 0))))
            (Utilities|Array|Clear _ownedfood)
            (Utilities|Array|Add _ownedfood _returnvalue))
          (:then_2
            ;[1 1 1] CPP
            (Class|TaskPawn|AddNewKitchenItemtoLevelItems _mytaskpawn (Utilities|GetDisplayName _returnvalue) "ITEM_JUICE_APPLE_GREEN" "IN_JUCIER" _cooktype)
            (Class|TaskPawn|AddKitchenItemAttribute _mytaskpawn "Juicer Container" (Utilities|GetDisplayName _returnvalue) _cooktype))
          (:then_3
            (Variables|Default|SetGreenAppleCount 0)
            (Variables|Default|SetbOccupied true)
            (CallFunction|InstrunctionUISetting))
          (:then_4
            (bind _asbp_cook_2 (Utilities|Casting|CastToBP_Cook (Game|GetPlayerCharacter 0)))
            (Class|TaskPawn|ClearAppleinJuicer (Variables|/Game/Blueprints/BP_Cook.BP_Cook_C|GetMyTaskPawn _asbp_cook_2))))))))

(event Custom|InstrunctionUISetting
  ;[1 1 1] UI Control
  (bind _as1_1_juicer_instruction (Utilities|Casting|CastTo1-1_Juicer_Instruction (UserInterface|GetUserWidgetObject (Variables|Default|GetInstructionWidget))))
  (if (Variables|Default|GetbOccupied)
    (Widget|SetVisibility (Variables|/Game/Blueprints/Kitchen3/1-1_Juicer_Instruction.1-1_Juicer_Instruction_C|GetHorizontalBox_Juice _as1_1_juicer_instruction) "Visible")
    (Widget|SetVisibility (Variables|/Game/Blueprints/Kitchen3/1-1_Juicer_Instruction.1-1_Juicer_Instruction_C|Geticon_1 _as1_1_juicer_instruction) "Hidden")
    (Widget|SetVisibility (Variables|/Game/Blueprints/Kitchen3/1-1_Juicer_Instruction.1-1_Juicer_Instruction_C|Geticon_2 _as1_1_juicer_instruction) "Hidden")
    (Widget|SetVisibility (Variables|/Game/Blueprints/Kitchen3/1-1_Juicer_Instruction.1-1_Juicer_Instruction_C|Geticon_3 _as1_1_juicer_instruction) "Hidden")
    (Widget|SetVisibility (Variables|/Game/Blueprints/Kitchen3/1-1_Juicer_Instruction.1-1_Juicer_Instruction_C|GetImage_1 _as1_1_juicer_instruction) "Hidden")
    (Widget|SetVisibility (Variables|/Game/Blueprints/Kitchen3/1-1_Juicer_Instruction.1-1_Juicer_Instruction_C|GetImage_2 _as1_1_juicer_instruction) "Hidden")
    (Widget|SetVisibility (Variables|/Game/Blueprints/Kitchen3/1-1_Juicer_Instruction.1-1_Juicer_Instruction_C|GetImage_3 _as1_1_juicer_instruction) "Hidden")
    (else
      (Widget|SetVisibility (Variables|/Game/Blueprints/Kitchen3/1-1_Juicer_Instruction.1-1_Juicer_Instruction_C|GetHorizontalBox_Juice _as1_1_juicer_instruction) "Collapsed")
      (switch int (Variables|Default|GetGreenAppleCount)
        (:0
          (Widget|SetVisibility (Variables|/Game/Blueprints/Kitchen3/1-1_Juicer_Instruction.1-1_Juicer_Instruction_C|Geticon_1 _as1_1_juicer_instruction) "Visible")
          (Widget|SetVisibility (Variables|/Game/Blueprints/Kitchen3/1-1_Juicer_Instruction.1-1_Juicer_Instruction_C|Geticon_2 _as1_1_juicer_instruction) "Visible")
          (Widget|SetVisibility (Variables|/Game/Blueprints/Kitchen3/1-1_Juicer_Instruction.1-1_Juicer_Instruction_C|Geticon_3 _as1_1_juicer_instruction) "Visible")
          (Widget|SetVisibility (Variables|/Game/Blueprints/Kitchen3/1-1_Juicer_Instruction.1-1_Juicer_Instruction_C|GetImage_1 _as1_1_juicer_instruction) "Hidden")
          (Widget|SetVisibility (Variables|/Game/Blueprints/Kitchen3/1-1_Juicer_Instruction.1-1_Juicer_Instruction_C|GetImage_2 _as1_1_juicer_instruction) "Hidden")
          (Widget|SetVisibility (Variables|/Game/Blueprints/Kitchen3/1-1_Juicer_Instruction.1-1_Juicer_Instruction_C|GetImage_3 _as1_1_juicer_instruction) "Hidden"))
        (:1
          (Widget|SetVisibility (Variables|/Game/Blueprints/Kitchen3/1-1_Juicer_Instruction.1-1_Juicer_Instruction_C|Geticon_1 _as1_1_juicer_instruction) "Hidden")
          (Widget|SetVisibility (Variables|/Game/Blueprints/Kitchen3/1-1_Juicer_Instruction.1-1_Juicer_Instruction_C|Geticon_2 _as1_1_juicer_instruction) "Visible")
          (Widget|SetVisibility (Variables|/Game/Blueprints/Kitchen3/1-1_Juicer_Instruction.1-1_Juicer_Instruction_C|Geticon_3 _as1_1_juicer_instruction) "Visible")
          (Widget|SetVisibility (Variables|/Game/Blueprints/Kitchen3/1-1_Juicer_Instruction.1-1_Juicer_Instruction_C|GetImage_1 _as1_1_juicer_instruction) "Visible")
          (Widget|SetVisibility (Variables|/Game/Blueprints/Kitchen3/1-1_Juicer_Instruction.1-1_Juicer_Instruction_C|GetImage_2 _as1_1_juicer_instruction) "Hidden")
          (Widget|SetVisibility (Variables|/Game/Blueprints/Kitchen3/1-1_Juicer_Instruction.1-1_Juicer_Instruction_C|GetImage_3 _as1_1_juicer_instruction) "Hidden"))
        (:2
          (Widget|SetVisibility (Variables|/Game/Blueprints/Kitchen3/1-1_Juicer_Instruction.1-1_Juicer_Instruction_C|Geticon_1 _as1_1_juicer_instruction) "Hidden")
          (Widget|SetVisibility (Variables|/Game/Blueprints/Kitchen3/1-1_Juicer_Instruction.1-1_Juicer_Instruction_C|Geticon_2 _as1_1_juicer_instruction) "Hidden")
          (Widget|SetVisibility (Variables|/Game/Blueprints/Kitchen3/1-1_Juicer_Instruction.1-1_Juicer_Instruction_C|Geticon_3 _as1_1_juicer_instruction) "Visible")
          (Widget|SetVisibility (Variables|/Game/Blueprints/Kitchen3/1-1_Juicer_Instruction.1-1_Juicer_Instruction_C|GetImage_1 _as1_1_juicer_instruction) "Visible")
          (Widget|SetVisibility (Variables|/Game/Blueprints/Kitchen3/1-1_Juicer_Instruction.1-1_Juicer_Instruction_C|GetImage_2 _as1_1_juicer_instruction) "Visible")
          (Widget|SetVisibility (Variables|/Game/Blueprints/Kitchen3/1-1_Juicer_Instruction.1-1_Juicer_Instruction_C|GetImage_3 _as1_1_juicer_instruction) "Hidden"))
        (:3
          (Widget|SetVisibility (Variables|/Game/Blueprints/Kitchen3/1-1_Juicer_Instruction.1-1_Juicer_Instruction_C|Geticon_1 _as1_1_juicer_instruction) "Hidden")
          (Widget|SetVisibility (Variables|/Game/Blueprints/Kitchen3/1-1_Juicer_Instruction.1-1_Juicer_Instruction_C|Geticon_2 _as1_1_juicer_instruction) "Hidden")
          (Widget|SetVisibility (Variables|/Game/Blueprints/Kitchen3/1-1_Juicer_Instruction.1-1_Juicer_Instruction_C|Geticon_3 _as1_1_juicer_instruction) "Hidden")
          (Widget|SetVisibility (Variables|/Game/Blueprints/Kitchen3/1-1_Juicer_Instruction.1-1_Juicer_Instruction_C|GetImage_1 _as1_1_juicer_instruction) "Visible")
          (Widget|SetVisibility (Variables|/Game/Blueprints/Kitchen3/1-1_Juicer_Instruction.1-1_Juicer_Instruction_C|GetImage_2 _as1_1_juicer_instruction) "Visible")
          (Widget|SetVisibility (Variables|/Game/Blueprints/Kitchen3/1-1_Juicer_Instruction.1-1_Juicer_Instruction_C|GetImage_3 _as1_1_juicer_instruction) "Visible")))
      (Default|PlayUIAnimation _as1_1_juicer_instruction))))

(event EventBeginPlay
  (|CallParentFunction)
  (CallFunction|InstrunctionUISetting))

(event EventTick
  (params (DeltaSeconds :type Float%20%28single-precision%29))
  (bind _ownedfood (Variables|Default|GetOwnedFood))
  (bind _output (Utilities|Array|Get(acopy) _ownedfood))
  ;[1 1 1] Conditions for Juice: bHolding in Juicer, Must Put In Bowl
  (if (> (Utilities|Array|Length _ownedfood) 0)
    (if (Variables|/Game/Blueprints/BP_PickupItem.BP_PickupItem_C|GetbHolding _output)
      (if (Variables|/Game/Blueprints/BP_Food.BP_Food_C|GetbMustPutInBowl _output)
        (Variables|Default|SetbOccupied false)
        (bind _asbp_cook (Utilities|Casting|CastToBP_Cook (Game|GetPlayerCharacter 0)))
        (Class|TaskPawn|RemoveItemAttributes (Variables|/Game/Blueprints/BP_Cook.BP_Cook_C|GetMyTaskPawn _asbp_cook) "Juicer Container")
        (Utilities|Array|Clear _ownedfood)
        (CallFunction|InstrunctionUISetting)))))

(fn ConstructionScript
  (|CallParentFunction))