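; Robot AI cook for a kitchen level that carries out actions assigned through MyTaskPawn.
; Tick switches on the task pawn's action: move to a target found by name, pick up or drop, or operate.
; When idle, it periodically finds an item within set bounds and requests moving it to the middle table.
; Failed navigation posts an apology, drops any held item and retreats near its start point.
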(event EventBeginPlay
  ;[1 1 1] Set Max Movement Speed for AI
  (|CallParentFunction)
  (Variables|/Script/Engine.CharacterMovementComponent|SetMaxWalkSpeed (Variables|Character|GetCharacterMovement self) 2.7e+02)
  (Variables|Default|SetCookType "ROBOT")
  (Variables|/Script/SimpleOvercooked.TaskPawn|SetAIAction (Variables|Default|GetMyTaskPawn) "IDLE")
  (Rendering|SetVisibility (Variables|Default|GetScene) false true)
  (Variables|Default|SetOriginalTransform (Transformation|GetActorTransform)))

(event Collision|EventActorBeginOverlap
  (params (OtherActor :type Actor%20Object%20Reference))
  (|CallParentFunction OtherActor) ; This node is disabled and will not be called.\nDrag off pins to build functionality.
)

(event EventTick
  (params (DeltaSeconds :type Float%20%28single-precision%29))
  (bind _self self)
  (bind _charactermovement (Variables|Character|GetCharacterMovement))
  (bind _mytaskpawn (Variables|Default|GetMyTaskPawn))
  (bind _aiaction (Variables|/Script/SimpleOvercooked.TaskPawn|GetAIAction _mytaskpawn))
  (bind _aitargetname (Variables|/Script/SimpleOvercooked.TaskPawn|GetAITargetName _mytaskpawn))
  (|CallParentFunction 0.0)
  (if (not (Variables|Default|GetInProgress))
    (switch Utilities|FlowControl|Switch|SwitchonEAIAction _aiaction
      (:IDLE
        (bind _output_get (Variables|Default|SetIdleTimePass (+ (Variables|Default|GetIdleTimePass) DeltaSeconds)))
        (if (> _output_get 1.5)
          (Variables|Default|SetIdleTimePass 0.0)
          (Utilities|FlowControl|Sequence
            (:then_0
              (bind _targetactor (CallFunction|FindPickItem2MiddleTable(1-2Only)))
              (if (!= _targetactor 0)
                (Class|TaskPawn|PickUpItem2MiddleTable (Variables|Default|GetMyTaskPawn) (Utilities|GetDisplayName _targetactor))
                (Development|PrintString (Utilities|String|EnumtoString _aiaction)))))))
      (:MOVE_TO
        (Variables|Default|SetNavTimePass (+ DeltaSeconds (Variables|Default|GetNavTimePass)))
        ;[1 1 1] Enable Movement
        (Components|Activation|SetActive _charactermovement true false)
        ;[1 1 1] Find Target Actor
        (bind _outactors (Actor|GetAllActorsOfClass "/Script/Engine.Actor"))
        (bind _array_element (Utilities|Array|ForEachLoopwithBreak _outactors :!label _label)
          (:LoopBody
            (if (Utilities|Enum|Equal(Enum) (Utilities|GetDisplayName _array_element) _aitargetname)
              (bind _output_get_2 (Variables|Default|SetTargetActor _array_element))
              (goto _label Break)))
          (:Completed
            ;[1 1 1] Check Actor Valid
            (if (Utilities|IsValid _output_get_2)
              ;[1 1 1] Move To Target
              (AI|AIMoveTo _self (Math|Vector|MakeVector (.X (Math|Vector|BreakVector (Transformation|GetActorLocation (Variables|Default|GetTargetActor)))) (.Y (Math|Vector|BreakVector (Transformation|GetActorLocation (Variables|Default|GetTargetActor)))) (.Z (Math|Vector|BreakVector (Transformation|GetActorLocation _self)))) 0 15.0 false
                (:then
                  ;[1 1 1] Look At Target Actor
                  (Transformation|SetActorRotation (Math|Rotator|MakeRotator 0.0 0.0 (.Yaw (Math|Rotator|BreakRotator (Math|Rotator|FindLookatRotation (Transformation|GetActorLocation) (Transformation|GetActorLocation (Variables|Default|GetTargetActor)))))) true)
                  ;[1 1 1] Navigation Succeed/Fail!
                  (if (> (Variables|Default|GetNavTimePass) 5.0)
                    (Variables|Default|SetNavTimePass 0.0 :!label _label_2)
                    (Variables|Default|SetInProgress true)
                    (Variables|/Script/SimpleOvercooked.TaskPawn|Setsuggestion (Variables|Default|GetMyTaskPawn) "SORRY, I CAN\"T GET THERE!!!!!!!!(>_<)")
                    ;[1 1 1] Update AI Action Plan: Fail     drop current item move to a random near-by point and replan
                    (if (!= (Variables|Default|GetCurrentItem) 0)
                      (CallFunction|AIPickUpDrop))
                    (Components|Activation|SetActive (Variables|Character|GetCharacterMovement) true false)
                    (AI|AIMoveTo self (.RandomLocation (AI|Navigation|GetRandomReachablePointinRadius (.Location (Math|Transform|BreakTransform (Variables|Default|GetOriginalTransform))) 2e+02 0 0)) 0 15.0 false)
                    (elif (or (Utilities|Enum|Equal(Enum) _aitargetname (Utilities|GetDisplayName (Variables|Default|GetCollisionActor))) (Utilities|Enum|Equal(Enum) (Utilities|GetDisplayName (Variables|Default|GetCurrentCookTool)) _aitargetname))
                      (Variables|Default|SetNavTimePass 0.0)))))
              (else
                (goto _label_2))))))
      (:PICK_UP_DROP
        (Variables|Default|SetInProgress true)
        (Components|Activation|SetActive _charactermovement false false)
        ;[1 1 1] PickUpDrop Item
        (Utilities|FlowControl|Delay 0.2)
        (CallFunction|AIPickUpDrop)
        (Utilities|FlowControl|Delay 0.2))
      (:INSPECT
        (Variables|Default|SetInProgress true)
        (Components|Activation|SetActive _charactermovement false false)
        ;[1 1 1] Cut/Operate Juicer
        (Utilities|FlowControl|Delay 0.2)
        (CallFunction|AIOperate)
        (Utilities|FlowControl|Delay 1.6)))))

(fn ConstructionScript
  (|CallParentFunction))

(fn FindPickItem2MiddleTable(1-2Only)
  (bind _outactors (Actor|GetAllActorsOfClass "/Script/Engine.Actor"))
  (bind _array_element (Utilities|Array|ForEachLoopwithBreak _outactors)
    (:LoopBody
      (bind _asbp_pickup_item (Utilities|Casting|CastToBP_PickupItem _array_element))
      (if (and (< (.X (Math|Vector|BreakVector (Transformation|GetActorLocation _asbp_pickup_item))) 4e+02) (> (.X (Math|Vector|BreakVector (Transformation|GetActorLocation _asbp_pickup_item))) 1.1e+02))
        (if (and (< (.Y (Math|Vector|BreakVector (Transformation|GetActorLocation _asbp_pickup_item))) 4.7e+02) (> (.Y (Math|Vector|BreakVector (Transformation|GetActorLocation _asbp_pickup_item))) -4.7e+02))
          (if (Math|Boolean|ANDBoolean (Utilities|Enum|NotEqual(Enum) (Variables|/Game/Blueprints/BP_PickupItem.BP_PickupItem_C|GetAbstractLocation _asbp_pickup_item) "ON_TABLE") (Utilities|Enum|NotEqual(Enum) (Variables|/Game/Blueprints/BP_PickupItem.BP_PickupItem_C|GetAbstractLocation _asbp_pickup_item) "IN_JUCIER") (Utilities|Enum|NotEqual(Enum) (Variables|/Game/Blueprints/BP_PickupItem.BP_PickupItem_C|GetAbstractLocation _asbp_pickup_item) "BE_HOLD"))
            (return _asbp_pickup_item)))))
    (:Completed
      (return 0))))