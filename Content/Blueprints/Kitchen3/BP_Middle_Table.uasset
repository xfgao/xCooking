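; BP_Middle_Table is a kitchen table that snaps a dropped pickup item onto its box and holds one item at a time.
; Box overlap freezes the item's physics, aligns it and marks it on-grid at the table.
; Tick frees the table once that item is held or off-grid.
; Both changes report table occupancy to the player cook's task pawn, with placement also reporting item location.
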(event OnComponentBeginOverlap(Box)
  (params (OverlappedComponent :type Primitive%20Component%20Object%20Reference) (OtherActor :type Actor%20Object%20Reference) (OtherComp :type Primitive%20Component%20Object%20Reference) (OtherBodyIndex :type Integer) (bFromSweep :type Boolean) (SweepResult :type Hit%20Result%20Structure%20%28by%20ref%29))
  (if (not (Variables|Default|GetbOccupied))
    (bind _asbp_pickup_item (Utilities|Casting|CastToBP_PickupItem OtherActor))
    (if (not (Variables|/Game/Blueprints/BP_PickupItem.BP_PickupItem_C|GetbHolding _asbp_pickup_item))
      (if (not (Variables|/Game/Blueprints/BP_PickupItem.BP_PickupItem_C|GetbOnGrid _asbp_pickup_item))
        (Physics|SetSimulatePhysics (Variables|/Game/Blueprints/BP_PickupItem.BP_PickupItem_C|GetStaticMesh _asbp_pickup_item) false)
        (Collision|SetCollisionEnabled (Variables|/Game/Blueprints/BP_PickupItem.BP_PickupItem_C|GetStaticMesh _asbp_pickup_item) "NoCollision")
        (Transformation|SetActorLocation _asbp_pickup_item (Transformation|GetWorldLocation (Variables|Default|GetBox)) false true)
        (Transformation|SetActorRotation _asbp_pickup_item (Transformation|GetActorRotation) true)
        (Variables|Default|SetbOccupied true)
        (Variables|/Game/Blueprints/BP_PickupItem.BP_PickupItem_C|SetbOnGrid _asbp_pickup_item true)
        (bind _output_get (Variables|Default|SetOccupiedItem _asbp_pickup_item))
        (Collision|SetCollisionEnabled (Variables|/Game/Blueprints/BP_PickupItem.BP_PickupItem_C|GetStaticMesh _asbp_pickup_item) "QueryAndPhysics")
        ;[1 1 1] Cpp: change occupation for table
        (bind _asbp_cook (Utilities|Casting|CastToBP_Cook (Game|GetPlayerCharacter 0)))
        (Class|TaskPawn|ChangeToolOccupation (Variables|/Game/Blueprints/BP_Cook.BP_Cook_C|GetMyTaskPawn _asbp_cook) (Utilities|GetDisplayName self) true)
        (Class|TaskPawn|ChangeItemAbstractLocation (Variables|/Game/Blueprints/BP_Cook.BP_Cook_C|GetMyTaskPawn _asbp_cook) (Utilities|GetDisplayName _output_get) "ON_TABLE")
        (Variables|/Game/Blueprints/BP_PickupItem.BP_PickupItem_C|SetAbstractLocation _output_get "ON_TABLE")
        (for _array_element (Variables|/Script/SimpleOvercooked.TaskPawn|GetLevelItems (Variables|/Game/Blueprints/BP_Cook.BP_Cook_C|GetMyTaskPawn _asbp_cook))
          (if (Utilities|Enum|Equal(Enum) (.item_name (Utilities|Struct|BreakKitchenItem _array_element)) (Utilities|GetDisplayName (Variables|Default|GetOccupiedItem)))
            _))))))

(event EventBeginPlay)

(event EventTick
  (params (DeltaSeconds :type Float%20%28single-precision%29))
  (if (!= (Variables|Default|GetOccupiedItem) 0)
    (if (or (Variables|/Game/Blueprints/BP_PickupItem.BP_PickupItem_C|GetbHolding (Variables|Default|GetOccupiedItem)) (not (Variables|/Game/Blueprints/BP_PickupItem.BP_PickupItem_C|GetbOnGrid (Variables|Default|GetOccupiedItem))))
      (Variables|Default|SetRecordItemName (Utilities|GetDisplayName (Variables|Default|GetOccupiedItem)))
      ;[1 1 1] Must be Pick Up: Location ON hold
      (Variables|/Game/Blueprints/BP_PickupItem.BP_PickupItem_C|SetAbstractLocation (Variables|Default|GetOccupiedItem) "UNKNOWN")
      (Variables|Default|SetOccupiedItem 0)
      ;[1 1 1] Cpp: change occupation for table
      (Variables|Default|SetbOccupied false)
      (bind _asbp_cook (Utilities|Casting|CastToBP_Cook (Game|GetPlayerCharacter 0)))
      (Class|TaskPawn|ChangeToolOccupation (Variables|/Game/Blueprints/BP_Cook.BP_Cook_C|GetMyTaskPawn _asbp_cook) (Utilities|GetDisplayName self) false))))

(fn ConstructionScript)